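; BP_IWeapon appears to be a Blueprint Interface declaring the shared contract for weapon and melee combat communication between objects.
; It exposes get/set pairs for weapon state, combat state and movement permission, plus a current-weapon getter and a weapon change call.
; Further functions cover health increase and decrease, sword grab and release, equip and unequip, hit and death.
; All functions are stubs returning defaults, with no logic here.
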(fn `GetWeapon_CanMove`
  (returns (CanMove :type Boolean))
  (return false))

(fn `GetWeapon_Combat`
  (returns (Combat :type "/Game/Enums/ECombatType Enum"))
  (return "NewEnumerator0"))

(fn `GetWeapon_Current`
  (returns (Result :type "/Game/Weapons/BP_Weapon Object Reference"))
  (return null))

(fn `GetWeapon_State`
  (returns (State :type "/Game/Enums/EStateType Enum"))
  (return "NewEnumerator0"))

(fn `SetWeapon_CanMove`
  (params (GetMove :type Boolean))
  (returns (Result :type Boolean))
  (return false))

(fn `SetWeapon_Combat`
  (params (Combat :type "/Game/Enums/ECombatType Enum" :default "NewEnumerator0"))
  (returns (Result :type "/Game/Enums/ECombatType Enum"))
  (return "NewEnumerator0"))

(fn `SetWeapon_State`
  (params (state :type "/Game/Enums/EStateType Enum" :default "NewEnumerator0"))
  (returns (Result :type "/Game/Enums/EStateType Enum"))
  (return "NewEnumerator0"))

(fn `Weapon_Change`
  (params (NewWeapon :type "/Game/Weapons/BP_Weapon Object Reference"))
  (returns (Weapon :type "/Game/Weapons/BP_Weapon Object Reference"))
  (return null))

(fn `Weapon_Dead`
  (returns (Result :type Boolean))
  (return false))

(fn `Weapon_DecreaseHealth`
  (params (Health :type "Float (double-precision)"))
  (returns (Result :type "Float (double-precision)"))
  (return 0.0))

(fn `Weapon_Equipped`
  (returns (Result :type Boolean))
  (return false))

(fn `Weapon_GrabSword`
  (returns (Result :type Boolean))
  (return false))

(fn `Weapon_Hitted`
  (returns (Result :type Boolean))
  (return false))

(fn `Weapon_IncreaseHealth`
  (params (Health :type "Float (double-precision)"))
  (returns (Result :type "Float (double-precision)"))
  (return 0.0))

(fn `Weapon_UnEquipped`
  (returns (Result :type Boolean))
  (return false))

(fn `Weapon_UnGrabSword`
  (returns (Result :type Boolean))
  (return false))