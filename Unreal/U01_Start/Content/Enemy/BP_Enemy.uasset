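; Enemy character that carries a spawned greatsword, shows a health bar widget and reacts to damage.
; AnyDamage reduces health, turns it to the attacker, flashes dynamic materials red and triggers the player's last-combo effect.
; Surviving hits play a reaction with sword knockback or a timed fireball burn; death plays a fall montage, then destroys enemy and sword.
; Weapon getters and setters are mostly simple pass-throughs or stubs.
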(event `self.ReceiveBeginPlay`
  (`|ExecutionSequence`
    (:`then_0`
      (bind _returnvalue (`|SpawnActorFromClass` "/Game/Weapons/Combo/BP_Sword.BP_Sword_C" (`KismetMathLibrary.MakeTransform` (0.0 0.0 0.0)) "Undefined" "OverrideRootScale" self null))
      (bind _output_get (set `self.Sword` _returnvalue))
      (`self.K2_AttachToComponent` _output_get (`self.Mesh`) "GreatSword" "KeepRelative" "KeepRelative" "KeepRelative" true))
    (:`then_1`
      (`self.UpdateHealthBar`))
    (:`then_2`
      (bind _returnvalue_2 (`KismetMaterialLibrary.CreateDynamicMaterialInstance` "/Game/Materials/M_UE4Man_Body_Inst_Enemy.M_UE4Man_Body_Inst_Enemy"))
      (`KismetArrayLibrary.Array_Add` (`self.Materials`) _returnvalue_2)
      (bind _returnvalue_3 (`KismetMaterialLibrary.CreateDynamicMaterialInstance` "/Game/Materials/M_UE4Man_ChestLogo_Inst_Enemy.M_UE4Man_ChestLogo_Inst_Enemy"))
      (`KismetArrayLibrary.Array_Add` (`self.Materials`) _returnvalue_3)
      (`PrimitiveComponent.SetMaterial` (`self.Mesh`) 0 (`|GetArrayItem` (`self.Materials`)))
      (`PrimitiveComponent.SetMaterial` (`self.Mesh`) 1 (`|GetArrayItem` (`self.Materials`) 1))
      (bind _returnvalue_4 (`KismetMaterialLibrary.CreateDynamicMaterialInstance` "/Game/Materials/M_Blade_BlackKnight_Inst_Enemy.M_Blade_BlackKnight_Inst_Enemy"))
      (`KismetArrayLibrary.Array_Add` (`self.Materials`) _returnvalue_4)
      (`PrimitiveComponent.SetMaterial` (`/Game/Weapons/Combo/BP_Sword.SkeletalMesh` (`self.Sword`)) 0 (`|GetArrayItem` (`self.Materials`) 2)))))

(event `self.ReceiveAnyDamage`
  (params (Damage :type "Float (single-precision)") (DamageType :type "DamageType Object Reference") (InstigatedBy :type "Controller Object Reference") (DamageCauser :type "Actor Object Reference"))
  (set `self.Causer` DamageCauser)
  (bind _ascharacter (cast `Character` (`Controller.K2_GetPawn` InstigatedBy)))
  (set `self.Attacker` _ascharacter)
  (set `self.Damage` Damage)
  (set `self.Health` (- (`self.Health`) (`self.Damage`)))
  (`self.UpdateHealthBar`)
  (`self.K2_SetActorRotation` (`KismetMathLibrary.FindLookAtRotation` (`self.K2_GetActorLocation`) (`self.K2_GetActorLocation` (`self.Attacker`))))
  (`self.ChangeMaterial` (struct :`R` 1.0 :`A` 1.0))
  (`KismetSystemLibrary.Delay` 0.2)
  (`self.ChangeMaterial` (struct :`R` 0.45098 :`G` 0.403922 :`B` 0.360784))
  (bind _asbp_player (cast `/Game/Player/BP_Player` (`self.Attacker`)))
  (`/Game/Player/BP_Player.PlayLastComboEffect` _asbp_player self)
  (if (<= (`self.Health`) 0.0)
    (`/Engine/EditorBlueprintResources/StandardMacros.DoOnce` false
      (:`Completed`
        (set `self.Dead` true)
        (`PrimitiveComponent.SetCollisionEnabled` (`self.CapsuleComponent`) "NoCollision")
        (`self.PlayAnimMontage` "/Game/Character/Montages/GetHitBackFall_Montage.GetHitBackFall_Montage" 1.2 "Start")
        (`KismetSystemLibrary.Delay` 5.0)
        (`self.K2_DestroyActor`)
        (`self.K2_DestroyActor` (`self.Sword`))))
    (else
      (`self.PlayAnimMontage` "/Game/Character/Montages/Hit_Reaction_Montage.Hit_Reaction_Montage" 2.0 "Default")
      (cast `/Game/Weapons/Combo/BP_Sword` (`self.Causer`)
        (:`then`
          (`self.K2_AddActorWorldOffset` (* (`KismetMathLibrary.Vector_Normal2D` (`self.GetActorForwardVector`)) (* (`CharacterMovementComponent.Mass` (`self.CharacterMovement`)) -0.2))))
        (:`CastFailed`
          (cast `/Game/Weapons/BP_FireBall` (`self.Causer`))
          (`ActorComponent.SetActive` (`self.Fire`) true false)
          (`KismetSystemLibrary.Delay` 5.0)
          (`ActorComponent.SetActive` (`self.Fire`) false false))))))

(fn `ChangeMaterial`
  (params (Color :type "LinearColor Structure"))
  (for _array_element (`self.Materials`)
    (`MaterialInstanceDynamic.SetVectorParameterValue` _array_element "BodyColor" (`local.Color`))))

(fn `GetWeapon_CanMove`
  (returns (CanMove :type Boolean))
  (return false))

(fn `GetWeapon_Combat`
  (returns (Combat :type "/Game/Enums/ECombatType Enum"))
  (return (`self.Combat`)))

(fn `GetWeapon_Current`
  (returns (Result :type "/Game/Weapons/BP_Weapon Object Reference"))
  (return null))

(fn `GetWeapon_State`
  (returns (State :type "/Game/Enums/EStateType Enum"))
  (return (`self.State`)))

(fn `SetWeapon_CanMove`
  (params (GetMove :type Boolean))
  (returns (Result :type Boolean))
  (return false))

(fn `SetWeapon_Combat`
  (params (Combat :type "/Game/Enums/ECombatType Enum" :default "NewEnumerator0"))
  (returns (Result :type "/Game/Enums/ECombatType Enum"))
  (bind _output_get (set `self.Combat` Combat))
  (return _output_get))

(fn `SetWeapon_State`
  (params (state :type "/Game/Enums/EStateType Enum" :default "NewEnumerator0"))
  (returns (Result :type "/Game/Enums/EStateType Enum"))
  (bind _output_get (set `self.State` state))
  (return _output_get))

(fn `UpdateHealthBar`
  (bind _aswb_health_bar (cast `/Game/Enemy/WB_HealthBar` (`WidgetComponent.GetUserWidgetObject` (`self.HealthBar`))))
  (`/Game/Enemy/WB_HealthBar.Update HealthBar` _aswb_health_bar (`self.Health`)))

(fn `UserConstructionScript`)

(fn `Weapon_Change`
  (params (NewWeapon :type "/Game/Weapons/BP_Weapon Object Reference"))
  (returns (Weapon :type "/Game/Weapons/BP_Weapon Object Reference"))
  (return null))