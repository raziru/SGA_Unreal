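; Player character with camera-relative movement, zoom, and Unarmed, Fist, Sword and Wizard combat modes; Jump becomes backstep or roll when armed.
; BeginPlay spawns the three weapon actors; mode switches set rotation style and the current Weapon that receives attacks.
; Wizard mode shows a slot widget and scroll-cycles heal, warp and throw skills.
; Lock-on sphere-traces enemies, picks by camera dot product, switches sideways by cross-product sign, and steers control rotation on Tick.
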(event `self.ReceiveBeginPlay`
  (`|ExecutionSequence`
    (:`then_0`
      (bind _returnvalue (`|SpawnActorFromClass` "/Game/Weapons/Combo/BP_Fist.BP_Fist_C" (`KismetMathLibrary.MakeTransform` (0.0 0.0 0.0)) "Undefined" "OverrideRootScale" self null))
      (bind _output_get (set `self.Fist` _returnvalue))
      (`self.K2_AttachToComponent` _output_get (`self.Mesh`) "None" "KeepRelative" "KeepRelative" "KeepRelative" true))
    (:`then_1`
      (bind _returnvalue_2 (`|SpawnActorFromClass` "/Game/Weapons/Combo/BP_Sword.BP_Sword_C" (`KismetMathLibrary.MakeTransform` (0.0 0.0 0.0)) "Undefined" "OverrideRootScale" self null))
      (bind _output_get_2 (set `self.Sword` _returnvalue_2))
      (`self.K2_AttachToComponent` _output_get_2 (`self.Mesh`) "Holster_Sword" "KeepRelative" "KeepRelative" "KeepRelative" true))
    (:`then_2`
      (bind _returnvalue_3 (`|SpawnActorFromClass` "/Game/Weapons/Wizard/BP_Wizard.BP_Wizard_C" (`KismetMathLibrary.MakeTransform` (0.0 0.0 0.0)) "Undefined" "OverrideRootScale" self null))
      (bind _output_get_3 (set `self.Wizard` _returnvalue_3))
      (`self.K2_AttachToComponent` _output_get_3 (`self.Mesh`) "Hand_FIreBall" "KeepRelative" "KeepRelative" "KeepRelative" true)
      (`self.SetActorHiddenInGame` (`self.Wizard`) true))
    (:`then_3`
      (set `self.Health` (`self.MaxHealth`)))
    (:`then_4`
      (`|ExecutionSequence`
        (:`then_0`
          (`KismetArrayLibrary.Array_Add` (`self.Skills`) (make `/Game/Weapons/Wizard/FWizardSkill` (`/Game/Weapons/Wizard/BP_Wizard.Heal` (`self.Wizard`)))))
        (:`then_1`
          (`KismetArrayLibrary.Array_Add` (`self.Skills`) (make `/Game/Weapons/Wizard/FWizardSkill` (`/Game/Weapons/Wizard/BP_Wizard.Warp` (`self.Wizard`)))))
        (:`then_2`
          (`KismetArrayLibrary.Array_Add` (`self.Skills`) (make `/Game/Weapons/Wizard/FWizardSkill` (`/Game/Weapons/Wizard/BP_Wizard.Throw` (`self.Wizard`)) "/Game/Weapons/Wizard/ThrowItems/BP_ThrowItem_FireBall.BP_ThrowItem_FireBall_C")))
        (:`then_3`
          (`KismetArrayLibrary.Array_Add` (`self.Skills`) (make `/Game/Weapons/Wizard/FWizardSkill` (`/Game/Weapons/Wizard/BP_Wizard.Throw` (`self.Wizard`)) "/Game/Weapons/Wizard/ThrowItems/BP_ThrowItem_IceBall.BP_ThrowItem_IceBall_C")))))
    (:`then_5`
      (bind _returnvalue_4 (`|CreateWidget` "/Game/Widgets/WB_Slots.WB_Slots_C" (`GameplayStatics.GetPlayerController` 0)))
      (bind _output_get_4 (set `self.Slots` _returnvalue_4))
      (`UserWidget.AddToViewport` _output_get_4 0)
      (`Widget.SetVisibility` (`self.Slots`) "Hidden"))))

(event `InputAxis|MoveForward`
  (params (AxisValue :type "Float (single-precision)"))
  (bind (_returnvalue_roll _returnvalue_pitch _returnvalue_yaw) (`KismetMathLibrary.BreakRotator` (`self.GetControlRotation`)))
  (if (`self.CanMove`)
    (`self.AddMovementInput` (`KismetMathLibrary.Vector_Normal2D` (`KismetMathLibrary.GetForwardVector` (`KismetMathLibrary.MakeRotator` 0.0 0.0 _returnvalue_yaw))) AxisValue)))

(event `InputAxis|MoveRight`
  (params (AxisValue :type "Float (single-precision)"))
  (bind (_returnvalue_roll _returnvalue_pitch _returnvalue_yaw) (`KismetMathLibrary.BreakRotator` (`self.GetControlRotation`)))
  (if (`self.CanMove`)
    (`self.AddMovementInput` (`KismetMathLibrary.Vector_Normal2D` (`KismetMathLibrary.GetRightVector` (`KismetMathLibrary.MakeRotator` 0.0 0.0 _returnvalue_yaw))) AxisValue)))

(event `InputAction|Walking`
  (params (Key :type "Key Structure"))
  (bind _charactermovement (`self.CharacterMovement`))
  (:`Pressed`
    (set `CharacterMovementComponent.MaxWalkSpeed` 300.0 _charactermovement))
  (:`Released`
    (set `CharacterMovementComponent.MaxWalkSpeed` 600.0 _charactermovement)))

(event `InputAction|Jump`
  (params (Key :type "Key Structure"))
  (:`Pressed`
    (if (`self.CanMove`)
      (if (`|EnumEquality` (`self.Combat`) "NewEnumerator0")
        (`self.Jump`)
        (else
          (`self.BackStep&Rolling`)))))
  (:`Released`
    (`self.StopJumping`)))

(event `BackStep&Rolling`
  (if (`self.IsStateIdle`)
    (if (< (`self.GetInputAxisValue`) 0.0)
      (set `self.State` "NewEnumerator5")
      (`self.PlayAnimMontage` "/Game/Character/Montages/BackStep_Montage.BackStep_Montage")
      (else
        (`|ExecutionSequence`
          (:`then_0`
            (set `self.State` "NewEnumerator7")
            (set `self.bUseControllerRotationYaw` false)
            (set `CharacterMovementComponent.bOrientRotationToMovement` true (`self.CharacterMovement`))
            (`CapsuleComponent.SetCapsuleSize` (`self.CapsuleComponent`) 34.0 44.0 true))
          (:`then_1`
            (`self.K2_SetActorRotation` (`self.GetRollDirection`)))
          (:`then_2`
            (`self.PlayAnimMontage` "/Game/Character/Montages/Roll_Montage.Roll_Montage")))))))

(event `End BackStep`
  (set `self.State` "NewEnumerator0"))

(event `End Rolling`
  (set `self.State` "NewEnumerator0")
  (if (not (`|EnumEquality` (`self.Combat`) "NewEnumerator0"))
    (set `self.bUseControllerRotationYaw` true)
    (set `CharacterMovementComponent.bOrientRotationToMovement` false (`self.CharacterMovement`))
    (`CapsuleComponent.SetCapsuleSize` (`self.CapsuleComponent`) 34.0 88.0 true)))

(event `InputAxis|VerticalLook`
  (params (AxisValue :type "Float (single-precision)"))
  (`self.AddControllerPitchInput` AxisValue))

(event `InputAxis|HorizontalLook`
  (params (AxisValue :type "Float (single-precision)"))
  (`self.AddControllerYawInput` AxisValue))

(event `InputAxis|Zoom`
  (params (AxisValue :type "Float (single-precision)"))
  (if (not (`|EnumEquality` (`self.Combat`) "NewEnumerator2"))
    (set `SpringArmComponent.TargetArmLength` (`KismetMathLibrary.FClamp` (+ (* AxisValue (`self.ZoomSpeed`)) (`SpringArmComponent.TargetArmLength` (`self.SpringArm`))) 100.0 600.0) (`self.SpringArm`))))

(event `InputAction|Attack`
  (params (Key :type "Key Structure"))
  (bind _weapon (`self.Weapon`))
  (:`Pressed`
    (`/Engine/EditorBlueprintResources/StandardMacros.IsValid` _weapon
      (:`Is Valid`
        (`/Game/Weapons/BP_Weapon.Attack` _weapon)))))

(event `PlayLastComboEffect`
  (params (Damager :type "Character Object Reference") (Effect :type "ParticleSystem Object Reference"))
  (if (`self.GetLastCombo`)
    (`GameplayStatics.SpawnEmitterAtLocation` Effect (`self.K2_GetActorLocation` Damager))))

(event `InputAction|Sword`
  (params (Key :type "Key Structure"))
  (:`Pressed`
    (if (`self.IsStateIdle`)
      (switch `/Game/Enums/ECombatType` (`self.Combat`)
        (:`NewEnumerator0`
          (`self.Equip Sword`))
        (:`NewEnumerator3`
          (`self.End Fist Mode`)
          (`self.Equip Sword`))
        (:`NewEnumerator1`
          (`self. Sheath sword`))
        (:`NewEnumerator2`
          (`self.End Wizard Mode`)
          (`self.Equip Sword`))))))

(event `Equip Sword`
  (set `self.State` "NewEnumerator2")
  (set `self.CanMove` false)
  (set `self.bUseControllerRotationYaw` true)
  (set `CharacterMovementComponent.bOrientRotationToMovement` false (`self.CharacterMovement`)))

(event `Equipped`
  (set `self.State` "NewEnumerator0")
  (set `self.CanMove` true)
  (set `self.Combat` "NewEnumerator1")
  (`self.Weapon_Change` (`self.Sword`)))

(event `Sheath sword`
  (set `self.State` "NewEnumerator3")
  (set `self.CanMove` false)
  (set `self.bUseControllerRotationYaw` false)
  (set `CharacterMovementComponent.bOrientRotationToMovement` true (`self.CharacterMovement`)))

(event `Sheathed Sword`
  (set `self.State` "NewEnumerator0")
  (set `self.CanMove` true)
  (set `self.Combat` "NewEnumerator0")
  (`self.Weapon_Change` null))

(event `Grab Sword`
  (`self.K2_AttachToComponent` (`self.Sword`) (`self.Mesh`) "Sword" "KeepRelative" "KeepRelative" "KeepRelative" true))

(event `UnGrab Sword`
  (`self.K2_AttachToComponent` (`self.Sword`) (`self.Mesh`) "Holster_Sword" "KeepRelative" "KeepRelative" "KeepRelative" true))

(event `InputAction|Wizard`
  (params (Key :type "Key Structure"))
  (:`Pressed`
    (if (`self.IsStateIdle`)
      (switch `/Game/Enums/ECombatType` (`self.Combat`)
        (:`NewEnumerator0`
          (`self.Start Wizard Mode`))
        (:`NewEnumerator3`
          (`self.End Fist Mode`)
          (`self.Start Wizard Mode`))
        (:`NewEnumerator1`
          (`self. Sheath sword`)
          (set `self.ChangeWizardMode` true))
        (:`NewEnumerator2`
          (`self.End Wizard Mode`))))))

(event `Start Wizard Mode`
  (set `self.Combat` "NewEnumerator2")
  (set `self.bUseControllerRotationYaw` true)
  (set `CharacterMovementComponent.bOrientRotationToMovement` false (`self.CharacterMovement`))
  (`self.SetActorHiddenInGame` (`self.Wizard`) false)
  (`self.Weapon_Change` (`self.Wizard`))
  (`Widget.SetVisibility` (`self.Slots`) "Visible")
  (`/Game/Widgets/WB_Slots.OnSeleted` (`self.Slots`) (`self.ScrollIndex`)))

(event `End Wizard Mode`
  (set `self.Combat` "NewEnumerator0")
  (set `self.bUseControllerRotationYaw` false)
  (set `CharacterMovementComponent.bOrientRotationToMovement` true (`self.CharacterMovement`))
  (`self.SetActorHiddenInGame` (`self.Wizard`) true)
  (`self.Weapon_Change` null)
  (`Widget.SetVisibility` (`self.Slots`) "Hidden"))

(event `SwordToWizardMode`
  (if (`self.ChangeWizardMode`)
    (set `self.ChangeWizardMode` false)
    (`self.Start Wizard Mode`)))

(event `InputAction|ScrollUp`
  (params (Key :type "Key Structure"))
  (bind (_output_skill _output_throwitemclass) (break `/Game/Weapons/Wizard/FWizardSkill` (`|GetArrayItem` (`self.Skills`) (`self.ScrollIndex`))))
  (bind _output_skill_2 (break `/Game/Weapons/Wizard/FWizardSkill` (`|GetArrayItem` (`self.Skills`) (`self.ScrollIndex`))))
  (bind _output_skill_3 (break `/Game/Weapons/Wizard/FWizardSkill` (`|GetArrayItem` (`self.Skills`) (`self.ScrollIndex`))))
  (:`Pressed`
    (switch `/Game/Enums/ECombatType` (`self.Combat`)
      (:`NewEnumerator2`
        (bind _result (`/Engine/EditorBlueprintResources/StandardMacros.IncrementInt` (`self.ScrollIndex`))
          (:`  `
            (set `self.ScrollIndex` (mod _result (`KismetArrayLibrary.Array_Length` (`self.Skills`))))
            (`/Game/Widgets/WB_Slots.OnSeleted` (`self.Slots`) (`self.ScrollIndex`) :!label _label)
            (bind _asbp_wizard_skill_throw (cast `/Game/Weapons/Wizard/BP_WizardSkill_Throw` _output_skill_2)
              (:`then`
                (`/Game/Weapons/Wizard/BP_Wizard.ChangeSkill` (`self.Wizard`) _output_skill)
                (`/Game/Weapons/Wizard/BP_WizardSkill_Throw.ChangeItem` _asbp_wizard_skill_throw _output_throwitemclass))
              (:`CastFailed`
                (`/Game/Weapons/Wizard/BP_Wizard.ChangeSkill` (`self.Wizard`) _output_skill_3)))))))))

(event `InputAction|ScrollDown`
  (params (Key :type "Key Structure"))
  (:`Pressed`
    (switch `/Game/Enums/ECombatType` (`self.Combat`)
      (:`NewEnumerator2`
        (bind _result (`/Engine/EditorBlueprintResources/StandardMacros.DecrementInt` (`self.ScrollIndex`))
          (:`  `
            (if (< _result 0)
              (set `self.ScrollIndex` (- (`KismetArrayLibrary.Array_Length` (`self.Skills`)) 1))
              (goto _label)
              (else
                (goto _label)))))))))

(event `Start FIst Mode`
  (set `self.Combat` "NewEnumerator3")
  (set `self.bUseControllerRotationYaw` true)
  (set `CharacterMovementComponent.bOrientRotationToMovement` false (`self.CharacterMovement`))
  (`self.Weapon_Change` (`self.Fist`)))

(event `End Fist Mode`
  (set `self.Combat` "NewEnumerator0")
  (set `self.bUseControllerRotationYaw` false)
  (set `CharacterMovementComponent.bOrientRotationToMovement` true (`self.CharacterMovement`))
  (`self.Weapon_Change` null))

(event `InputAction|Fist`
  (params (Key :type "Key Structure"))
  (:`Pressed`
    (if (`self.IsStateIdle`)
      (switch `/Game/Enums/ECombatType` (`self.Combat`)
        (:`NewEnumerator0`
          (`self.Start FIst Mode`))
        (:`NewEnumerator3`
          (`self.End Fist Mode`))
        (:`NewEnumerator1`
          (`self. Sheath sword`)
          (set `self.ChangeFistMode` true))
        (:`NewEnumerator2`
          (`self.End Wizard Mode`)
          (`self.Start FIst Mode`))))))

(event `SwordToFistMode`
  (if (`self.ChangeFistMode`)
    (set `self.ChangeFistMode` false)
    (`self.Start FIst Mode`)))

(event `InputAction|Targeting`
  (params (Key :type "Key Structure"))
  (:`Pressed`
    (if (`self.LockOnTarget`)
      (`self.EndLockOn`)
      (`self.SetTargetCursor` null)
      (elif (`|EnumInequality` (`self.Combat`) "NewEnumerator0")
        (`self.StartLockOn`)))))

(event `StartLockOn`
  (`self.GetTraceTargets`)
  (bind _enemy (`self.GetTargetEnemy`))
  (`/Engine/EditorBlueprintResources/StandardMacros.IsValid` _enemy
    (:`Is Valid`
      (set `self.LockOnEnemy` _enemy)
      (set `self.LockOnTarget` true))))

(event `EndLockOn`
  (set `self.LockOnEnemy` null)
  (set `self.LockOnTarget` false))

(event `TickLockOn`
  (if (`self.LockOnTarget`)
    (`/Engine/EditorBlueprintResources/StandardMacros.IsValid` (`self.LockOnEnemy`)
      (:`Is Valid`
        (`Controller.SetControlRotation` (`self.GetController`) (`KismetMathLibrary.FindLookAtRotation` (`self.K2_GetActorLocation`) (`self.K2_GetActorLocation` (`self.LockOnEnemy`)))))
      (:`Is Not Valid`
        (`self.EndLockon`)))))

(event `InputAction|TargetLeft`
  (params (Key :type "Key Structure"))
  (:`Pressed`
    (`self.GetNearestEnemy` false)))

(event `InputAction|TargetRight`
  (params (Key :type "Key Structure"))
  (:`Pressed`
    (`self.GetNearestEnemy` true)))

(event `self.ReceiveTick`
  (params (DeltaSeconds :type "Float (single-precision)"))
  (`self.TickLockOn`))

(fn `GetLastCombo`
  (returns (Result :type Boolean))
  (bind _asbp_combo (cast `/Game/Weapons/Combo/BP_Combo` (`self.Weapon`)))
  (return (`/Game/Weapons/Combo/BP_Combo.LastCombo` _asbp_combo)))

(fn `GetNearestEnemy`
  (params (`Is Right` :type Boolean))
  (locals (Map :type "Map of Float (double-precision) to /Game/Enemy/BP_Enemy Object Reference") (Distance :type "Float (double-precision)") (Minimum :type "Float (double-precision)" :default 10000000.0) (MnimumEnemy :type "/Game/Enemy/BP_Enemy Object Reference"))
  (bind _returnvalue (`self.K2_GetActorRotation`))
  (`/Engine/EditorBlueprintResources/StandardMacros.IsValid` (`self.LockOnEnemy`)
    (:`Is Valid`
      (for _array_element (`self.TargetEnemies`)
        (if (!= (`self.LockOnEnemy`) _array_element)
          (`BlueprintMapLibrary.Map_Add` (`local.Map`) (`KismetMathLibrary.Dot_VectorVector` (`KismetMathLibrary.GetUpVector` _returnvalue) (`KismetMathLibrary.Cross_VectorVector` (`KismetMathLibrary.GetForwardVector` _returnvalue) (- (`self.K2_GetActorLocation` _array_element) (`self.K2_GetActorLocation`)))) _array_element)))
      (bind _keys (`BlueprintMapLibrary.Map_Keys` (`local.Map`)))
      (for _array_element_2 _keys
        (set `local.Distance` _array_element_2)
        (if (`local.Is Right`)
          (if (> (`local.Distance`) 0.0)
            (if (<= (`KismetMathLibrary.Abs` (`local.Distance`)) (`local.Minimum`)) :!label _label
              (set `local.Minimum` (`local.Distance`))
              (set `local.MnimumEnemy` (`BlueprintMapLibrary.Map_Find` (`local.Map`) (`local.Distance`)))))
          (elif (< (`local.Distance`) 0.0)
            (goto _label))))
      (`self.SetTargetCursor` (`local.MnimumEnemy`))
      (set `self.LockOnEnemy` (`local.MnimumEnemy`)))))

(fn `GetRollDirection`
  (returns (ReturnValue :type "Rotator Structure"))
  (return (`KismetMathLibrary.FindLookAtRotation` (`self.K2_GetActorLocation`) (+ (`self.K2_GetActorLocation`) (`KismetMathLibrary.Vector_Normal2D` (`self.GetVelocity`))))))

(fn `GetTargetEnemy`
  (returns (Enemy :type "/Game/Enemy/BP_Enemy Object Reference"))
  (locals (Angle :type "Float (double-precision)" :default -2.0) (Result :type "/Game/Enemy/BP_Enemy Object Reference"))
  (for _array_element (`self.TargetEnemies`)
    (bind _returnvalue (`self.GetDotProductTo` (`GameplayStatics.GetPlayerCameraManager` 0) _array_element))
    (if (>= _returnvalue (`local.Angle`))
      (set `local.Angle` _returnvalue)
      (set `local.Result` _array_element)))
  (`self.SetTargetCursor` (`local.Result`))
  (return (`local.Result`)))

(fn `GetTraceTargets`
  (bind _returnvalue (`self.K2_GetActorLocation`))
  (bind _outhits (`KismetSystemLibrary.SphereTraceMultiForObjects` :`Start` _returnvalue :`End` (+ _returnvalue (`self.LockDistance`)) :`Radius` (`self.LockDistance`) :`ObjectTypes` (`|MakeArray` "ObjectTypeQuery3" :!type "EObjectTypeQuery Enum") :`DrawDebugType` "ForDuration" :`TraceColor` (struct :`R` 0.144904 :`G` 1.0 :`A` 1.0) :`TraceHitColor` (struct :`R` 1.0 :`G` 0.017847 :`A` 1.0) :`DrawTime` 2.0))
  (for _array_element _outhits
    (bind _asbp_enemy (cast `/Game/Enemy/BP_Enemy` (`.HitActor` (`GameplayStatics.BreakHitResult` _array_element))))
    (`KismetArrayLibrary.Array_AddUnique` (`self.TargetEnemies`) _asbp_enemy))
  (for _ (`self.TargetEnemies`)
    _))

(fn `GetWeapon_CanMove`
  (returns (CanMove :type Boolean))
  (return (`self.CanMove`)))

(fn `GetWeapon_Combat`
  (returns (Combat :type "/Game/Enums/ECombatType Enum"))
  (return (`self.Combat`)))

(fn `GetWeapon_Current`
  (returns (Result :type "/Game/Weapons/BP_Weapon Object Reference"))
  (return (`self.Weapon`)))

(fn `GetWeapon_State`
  (returns (State :type "/Game/Enums/EStateType Enum"))
  (return (`self.State`)))

(fn `IsStateIdle`
  (returns (`Can Equip` :type Boolean))
  (return (`|EnumEquality` (`self.State`) "NewEnumerator0")))

(fn `SetLastCombo`
  (params (LastCombo :type Boolean))
  (bind _asbp_combo (cast `/Game/Weapons/Combo/BP_Combo` (`self.Weapon`)))
  (set `/Game/Weapons/Combo/BP_Combo.LastCombo` LastCombo _asbp_combo)
  (return))

(fn `SetTargetCursor`
  (params (Enemy :type "/Game/Enemy/BP_Enemy Object Reference"))
  (for _array_element (`self.TargetEnemies`)
    (if (== (`local.Enemy`) _array_element)
      (bind _cursor (`/Game/Enemy/BP_Enemy.Cursor` _array_element))
      (`SceneComponent.SetVisibility` _cursor true false)
      (else
        (`SceneComponent.SetVisibility` _cursor false false)))))

(fn `SetWeapon_CanMove`
  (params (GetMove :type Boolean))
  (returns (Result :type Boolean))
  (bind _output_get (set `self.CanMove` GetMove))
  (return _output_get))

(fn `SetWeapon_Combat`
  (params (Combat :type "/Game/Enums/ECombatType Enum" :default "NewEnumerator0"))
  (returns (Result :type "/Game/Enums/ECombatType Enum"))
  (bind _output_get (set `self.Combat` Combat))
  (return _output_get))

(fn `SetWeapon_State`
  (params (state :type "/Game/Enums/EStateType Enum" :default "NewEnumerator0"))
  (returns (Result :type "/Game/Enums/EStateType Enum"))
  (bind _output_get (set `self.State` state))
  (return _output_get))

(fn `UserConstructionScript`)

(fn `Weapon_Change`
  (params (NewWeapon :type "/Game/Weapons/BP_Weapon Object Reference"))
  (returns (Weapon :type "/Game/Weapons/BP_Weapon Object Reference"))
  (if (!= (`self.Weapon`) NewWeapon)
    (`/Engine/EditorBlueprintResources/StandardMacros.IsValid` (`self.Weapon`)
      (:`Is Valid`
        (`/Game/Weapons/BP_Weapon.OffSelected` (`self.Weapon`)))
      (:`Is Not Valid`
        _))
    (`/Engine/EditorBlueprintResources/StandardMacros.IsValid` NewWeapon
      (:`Is Valid`
        (bind _output_get (set `self.Weapon` NewWeapon))
        (`/Game/Weapons/BP_Weapon.OnSelected` _output_get)
        (return _output_get))
      (:`Is Not Valid`
        (bind _output_get_2 (set `self.Weapon` null))
        (return _output_get_2)))))

(fn `Weapon_DecreaseHealth`
  (params (Health :type "Float (double-precision)"))
  (returns (Result :type "Float (double-precision)"))
  (bind _output_get (set `self.Health` (`KismetMathLibrary.FClamp` (- (`self.Health`) Health) 0.0 (`self.MaxHealth`))))
  (return _output_get))

(fn `Weapon_IncreaseHealth`
  (params (Health :type "Float (double-precision)"))
  (returns (Result :type "Float (double-precision)"))
  (bind _output_get (set `self.Health` (`KismetMathLibrary.FClamp` (+ Health (`self.Health`)) 0.0 (`self.MaxHealth`))))
  (return _output_get))