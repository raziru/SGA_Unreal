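; BP_09_Sound3D is a trigger actor that demonstrates 3D sound attenuation with a repeating dirt footstep cue.
; When BP_Player enters its Box, it draws green inner and red outer debug spheres and starts a looping timer that plays the cue at the actor's location with SA_Stepdirt attenuation.
; After PlayTime, a Delay clears the timer and resets the Play flag, which blocks retriggering during playback.
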(event `self.Box.OnComponentBeginOverlap`
  (params (OverlappedComponent :type "PrimitiveComponent Object Reference") (OtherActor :type "Actor Object Reference") (OtherComp :type "PrimitiveComponent Object Reference") (OtherBodyIndex :type Integer) (bFromSweep :type Boolean) (SweepResult :type "HitResult Structure (by ref)"))
  (cast `/Game/Player/BP_Player` OtherActor)
  (if (not (`self.Play`))
    (set `self.Play` true)
    (`KismetSystemLibrary.DrawDebugSphere` (`self.K2_GetActorLocation`) 400.0 12 (struct :`G` 1.0 :`A` 1.0) (`self.PlayTime`))
    (`KismetSystemLibrary.DrawDebugSphere` (`self.K2_GetActorLocation`) 1000.0 12 (struct :`R` 1.0 :`A` 1.0) (`self.PlayTime`))
    (bind _returnvalue (`KismetSystemLibrary.K2_SetTimerDelegate` (delegate `PlaySound`) 0.5 true))
    (set `self.TimerHandle` _returnvalue)
    (`KismetSystemLibrary.Delay` (`self.PlayTime`))
    (`KismetSystemLibrary.K2_ClearAndInvalidateTimerHandle` (`self.TimerHandle`))
    (set `self.Play` false)))

(event `PlaySound`
  (`GameplayStatics.PlaySoundAtLocation` "/Game/Sounds/S_Stepdirt_Cue.S_Stepdirt_Cue" (`self.K2_GetActorLocation`) (struct) 1.0 1.0 0.0 "/Game/Sounds/SA_Stepdirt.SA_Stepdirt" null null))

(fn `UserConstructionScript`)