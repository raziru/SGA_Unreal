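; Trigger actor that switches a point light on while something overlaps it.
; On begin play it hides the PointLight and applies the LightColor variable to it.
; Overlap begin shows the light and overlap end hides it again, with no filter on which actor overlaps and no count of overlapping actors.
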(event `self.ReceiveBeginPlay`
  (`SceneComponent.SetVisibility` (`self.PointLight`) false false)
  (`LightComponent.SetLightColor` (`self.PointLight`) (`self.LightColor`) true))

(event `self.ReceiveActorBeginOverlap`
  (params (OtherActor :type "Actor Object Reference"))
  (`SceneComponent.SetVisibility` (`self.PointLight`) true false))

(event `self.ReceiveActorEndOverlap`
  (params (OtherActor :type "Actor Object Reference"))
  (`SceneComponent.SetVisibility` (`self.PointLight`) false false))

(fn `UserConstructionScript`)