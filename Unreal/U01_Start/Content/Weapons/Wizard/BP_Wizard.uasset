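; BP_Wizard is the wizard weapon, which casts a skill through its owning character.
; On BeginPlay it sets its combat type, spawns a heal skill actor, attaches it to the character's Hand_FireBall mesh socket and makes it the active Skill.
; Attack, when allowed, changes state, plays the wizard attack montage and calls Spell on the skill; EndAttack resets state and calls EndSpell.
; Select and deselect events only print debug text.
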(event `self.OnSelected`
  (`KismetSystemLibrary.PrintString` "wizard"))

(event `self.OffSelected`
  (`KismetSystemLibrary.PrintString` "wizrd sheath"))

(event `self.ReceiveBeginPlay`
  (set `self.CombatType` "NewEnumerator2")
  (`|ExecutionSequence`
    (:`then_0`
      (bind _returnvalue (`|SpawnActorFromClass` "/Game/Weapons/Wizard/BP_WizardSkill_Heal.BP_WizardSkill_Heal_C" (`KismetMathLibrary.MakeTransform` (0.0 0.0 0.0)) "Undefined" "OverrideRootScale" self null))
      (set `self.Heal` _returnvalue)
      (bind _ascharacter (cast `Character` (`self.GetOwner`)))
      (`self.K2_AttachToComponent` (`self.Heal`) (`Character.Mesh` _ascharacter) "Hand_FireBall" "KeepRelative" "KeepRelative" "KeepRelative" true)
      (set `self.Skill` (`self.Heal`)))))

(event `self.Attack`
  (if (and (`self.CanAttack`) (`KismetSystemLibrary.IsValid` (`self.Skill`)))
    (`self.SetState` "NewEnumerator4")
    (bind _ascharacter (cast `Character` (`self.GetOwner`)))
    (`Character.PlayAnimMontage` _ascharacter "/Game/Character/Montages/Wizard_Attack_1_Montage.Wizard_Attack_1_Montage" 1.0 "None")
    (`/Game/Weapons/Wizard/BP_WizardSkill.Spell` (`self.Skill`))))

(event `self.EndAttack`
  (`self.SetState` "NewEnumerator0")
  (`/Game/Weapons/Wizard/BP_WizardSkill.EndSpell` (`self.Skill`)))

(fn `UserConstructionScript`)