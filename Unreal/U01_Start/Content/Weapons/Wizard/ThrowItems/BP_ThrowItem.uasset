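; Thrown-item actor for the Wizard's throw skill, providing shared hit handling with no active event logic of its own.
; Helper functions walk the owner chain from the item to BP_WizardSkill_Throw, then to BP_Wizard.
; BeginOverlap copies Power onto the wizard and delegates damage to its SendDamage.
; On success, it spawns the supplied explosion emitter at an offset from the hit actor and destroys the item.
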(fn `BeginOverlap`
  (params (OtherActor :type "Actor Object Reference") (Explosion :type "ParticleSystem Object Reference") (Location :type "Vector Structure") (Scale :type "Vector Structure") (Rotation :type "Rotator Structure"))
  (set `/Game/Weapons/BP_Weapon.Power` (`self.Power`) (`self.GetOwnerToWizrad`))
  (bind _result (`/Game/Weapons/BP_Weapon.SendDamage` (`self.GetOwnerToWizrad`) (`local.OtherActor`)))
  (if _result
    (`GameplayStatics.SpawnEmitterAtLocation` (`local.Explosion`) (+ (`local.Location`) (`self.K2_GetActorLocation` (`local.OtherActor`))) (`local.Rotation`) (`local.Scale`))
    (`self.K2_DestroyActor`)))

(fn `GetOwnerToThrow`
  (returns (`AsBP Wizard Skill Throw` :type "/Game/Weapons/Wizard/BP_WizardSkill_Throw Object Reference"))
  (bind _asbp_wizard_skill_throw (cast `/Game/Weapons/Wizard/BP_WizardSkill_Throw` (`self.GetOwner`)))
  (return _asbp_wizard_skill_throw))

(fn `GetOwnerToWizrad`
  (returns (`AsBP Wizard` :type "/Game/Weapons/Wizard/BP_Wizard Object Reference"))
  (bind _asbp_wizard (cast `/Game/Weapons/Wizard/BP_Wizard` (`self.GetOwner` (`self.GetOwnerToThrow`))))
  (return _asbp_wizard))

(fn `UserConstructionScript`)