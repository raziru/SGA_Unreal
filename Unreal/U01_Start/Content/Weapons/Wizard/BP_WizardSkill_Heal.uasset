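; BP_WizardSkill_Heal is the Wizard's Heal skill, handling the cast animation and movement lock.
; Spell disables the wizard's movement, then casts the wizard's owner to BP_Player and plays Wizard_Heal_Montage on it.
; EndSpell is a virtual override that re-enables movement.
; The Blueprint itself applies no healing and does not call EndSpell.
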(event `self.Spell`
  (`/Game/Weapons/BP_Weapon.SetCanMove` (`self.GetOwnerToWizard`) false)
  (bind _asbp_player (cast `/Game/Player/BP_Player` (`self.GetOwner` (`self.GetOwnerToWizard`))))
  (`Character.PlayAnimMontage` _asbp_player "/Game/Character/Montages/Wizard_Heal_Montage.Wizard_Heal_Montage" 1.0 "None"))

(event `self.EndSpell`
  (`/Game/Weapons/BP_Weapon.SetCanMove` (`self.GetOwnerToWizard`) true))

(fn `UserConstructionScript`
  (`parent.UserConstructionScript`))