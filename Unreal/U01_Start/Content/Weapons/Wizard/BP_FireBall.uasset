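; BP_FireBall is a wizard weapon fireball actor that damages characters it overlaps and expires after a short lifespan.
; Its sphere overlap identifies walls by a "Wall" substring in the display name, spawning an explosion without destroying the fireball.
; Characters other than the owner take Power damage credited to the owner's controller, then a second explosion effect spawns and the fireball destroys itself.
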(event `self.ReceiveBeginPlay`
  (`self.SetLifeSpan` 3.0))

(event `self.Sphere.OnComponentBeginOverlap`
  (params (OverlappedComponent :type "PrimitiveComponent Object Reference") (OtherActor :type "Actor Object Reference") (OtherComp :type "PrimitiveComponent Object Reference") (OtherBodyIndex :type Integer) (bFromSweep :type Boolean) (SweepResult :type "HitResult Structure (by ref)"))
  (if (`KismetStringLibrary.Contains` (`KismetSystemLibrary.GetDisplayName` OtherActor) "Wall")
    (`GameplayStatics.SpawnEmitterAtLocation` "/Game/Effects/P_Explosion1.P_Explosion1" (`self.K2_GetActorLocation`))
    (elif (!= OtherActor (`self.GetOwner`))
      (bind _ascharacter (cast `Character` OtherActor))
      (`GameplayStatics.ApplyDamage` _ascharacter (`self.Power`) (`self.GetInstigatorController` (`self.GetOwner`)) self)
      (`GameplayStatics.SpawnEmitterAtLocation` "/Game/Effects/P_Explosion2.P_Explosion2" (`self.K2_GetActorLocation` _ascharacter))
      (`self.K2_DestroyActor`))))

(fn `UserConstructionScript`)