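; BP_Fist is an unarmed melee weapon, filed with the combo weapons, that turns the owner's hands and feet into hitboxes.
; On BeginPlay it attaches four sphere components to fist sockets on the owning Character's mesh and disables their collision.
; OnCollision and OffCollision toggle collision on all its sphere components, and any sphere overlap calls SendDamage on the other actor.
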(event `self.ReceiveBeginPlay`
  (`parent.ReceiveBeginPlay`)
  (`self.AttachToSocket` (`self.LeftHand`) "Fist_LeftHand")
  (`self.AttachToSocket` (`self.RightHand`) "Fist_RightHand")
  (`self.AttachToSocket` (`self.LeftFoot`) "Fist_LeftFoot")
  (`self.AttachToSocket` (`self.RightFoot`) "Fist_RightFoot")
  (`self.Off Collision`))

(event `self.On Collision`
  (`self.SetCollsion` "QueryAndPhysics"))

(event `self.Off Collision`
  (`self.SetCollsion` "NoCollision"))

(event `self.RightHand.OnComponentBeginOverlap`
  (params (OverlappedComponent :type "PrimitiveComponent Object Reference") (OtherActor :type "Actor Object Reference") (OtherComp :type "PrimitiveComponent Object Reference") (OtherBodyIndex :type Integer) (bFromSweep :type Boolean) (SweepResult :type "HitResult Structure (by ref)"))
  (`self.SendDamage` OtherActor))

(event `self.RightFoot.OnComponentBeginOverlap`
  (params (OverlappedComponent :type "PrimitiveComponent Object Reference") (OtherActor :type "Actor Object Reference") (OtherComp :type "PrimitiveComponent Object Reference") (OtherBodyIndex :type Integer) (bFromSweep :type Boolean) (SweepResult :type "HitResult Structure (by ref)"))
  (`self.SendDamage` OtherActor))

(event `self.LeftFoot.OnComponentBeginOverlap`
  (params (OverlappedComponent :type "PrimitiveComponent Object Reference") (OtherActor :type "Actor Object Reference") (OtherComp :type "PrimitiveComponent Object Reference") (OtherBodyIndex :type Integer) (bFromSweep :type Boolean) (SweepResult :type "HitResult Structure (by ref)"))
  (`self.SendDamage` OtherActor))

(event `self.LeftHand.OnComponentBeginOverlap`
  (params (OverlappedComponent :type "PrimitiveComponent Object Reference") (OtherActor :type "Actor Object Reference") (OtherComp :type "PrimitiveComponent Object Reference") (OtherBodyIndex :type Integer) (bFromSweep :type Boolean) (SweepResult :type "HitResult Structure (by ref)"))
  (`self.SendDamage` OtherActor))

(fn `AttachToSocket`
  (params (Sphere :type "SphereComponent Object Reference") (`Socket Name` :type Name))
  (bind _ascharacter (cast `Character` (`self.GetOwner`)))
  (`SceneComponent.K2_AttachToComponent` (`local.Sphere`) (`Character.Mesh` _ascharacter) (`local.Socket Name`) "KeepRelative" "KeepRelative" "KeepRelative" true))

(fn `SetCollsion`
  (params (Type :type "ECollisionEnabled Enum" :default "NoCollision"))
  (for _array_element (`self.K2_GetComponentsByClass` "/Script/Engine.SphereComponent")
    (`PrimitiveComponent.SetCollisionEnabled` _array_element (`local.Type`))))

(fn `UserConstructionScript`
  (`parent.UserConstructionScript`))