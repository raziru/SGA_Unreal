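; BP_Combo is a combo attack weapon that plays a chain of montages on its owning Character.
; BeginPlay loads each ComboTable row, which defines montage, play rate, start section and movement permission.
; Attack starts the chain, or queues the next step while EnableNextCombo is open, closing it against repeated clicks.
; PlayNextCombo plays queued steps and flags the last one; EndAttack resets state, movement and combo progress.
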(event `self.ReceiveBeginPlay`
  ;[1 1 1] BeginPlay
  (bind _outrownames (`DataTableFunctionLibrary.GetDataTableRowNames` (`self.ComboTable`)))
  (for _array_element _outrownames
    (bind _returnvalue (`|GetDataTableRow` (`self.ComboTable`) _array_element)
      (:`then`
        (`KismetArrayLibrary.Array_Add` (`self.ComboMontages`) _returnvalue)))))

(event `self.Attack`
  ;[1 1 1] Attack
  (if (`self.EnableNextCombo`)
    (`/Engine/EditorBlueprintResources/StandardMacros.IncrementInt` (`self.ComboCount`)
      (:`  `
        (set `self.ExistNextCombo` true)
        (set `self.EnableNextCombo` false) ; 연타클릭 방지
      ))
    (elif (`self.CanAttack`)
      (`self.SetState` "NewEnumerator1")
      (`self.PlayComboMontage`))))

(event `PlayNextCombo`
  ;[1 1 1] ComboAttack
  (if (`self.ExistNextCombo`)
    (`self.PlayComboMontage`)
    (set `self.ExistNextCombo` false)
    (set `self.LastCombo` (== (- (`KismetArrayLibrary.Array_Length` (`self.ComboMontages`)) 1) (`self.ComboCount`)))))

(event `self.EndAttack`
  ;[1 1 1] EndAttack
  (`self.SetState` "NewEnumerator0")
  (`self.SetCanMove` true)
  (set `self.ComboCount` 0)
  (set `self.ExistNextCombo` false)
  (set `self.LastCombo` false))

(event `On Collision`)

(event `Off Collision`)

(fn `PlayComboMontage`
  (bind (_output_montage _output_playrate _output_startsectionname _output_canmove) (break `/Game/Weapons/Combo/FComboMontage` (`|GetArrayItem` (`self.ComboMontages`) (`self.ComboCount`))))
  (bind _ascharacter (cast `Character` (`self.GetOwner`)))
  (`Character.PlayAnimMontage` _ascharacter _output_montage _output_playrate _output_startsectionname)
  (`self.SetCanMove` _output_canmove))

(fn `UserConstructionScript`)