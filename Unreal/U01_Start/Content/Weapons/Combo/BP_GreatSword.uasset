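; BP_GreatSword is a great sword weapon Blueprint that deals damage through a Capsule hit volume.
; Its OnCollision and OffCollision events enable and disable the capsule's collision, which starts off at BeginPlay.
; Any actor that begins overlapping the capsule is passed to SendDamage.
; The select and deselect events only print debug strings.
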(event `self.OnSelected`
  (`KismetSystemLibrary.PrintString` "Sword"))

(event `self.OffSelected`
  (`KismetSystemLibrary.PrintString` "Sword Sheath"))

(event `self.ReceiveBeginPlay`
  (`parent.ReceiveBeginPlay`) ; __super::BeginPlay
  (`self.Off Collision`))

(event `self.Capsule.OnComponentBeginOverlap`
  (params (OverlappedComponent :type "PrimitiveComponent Object Reference") (OtherActor :type "Actor Object Reference") (OtherComp :type "PrimitiveComponent Object Reference") (OtherBodyIndex :type Integer) (bFromSweep :type Boolean) (SweepResult :type "HitResult Structure (by ref)"))
  (`self.SendDamage` OtherActor))

(event `self.On Collision`
  (`PrimitiveComponent.SetCollisionEnabled` (`self.Capsule`) "QueryAndPhysics"))

(event `self.Off Collision`
  (`parent.Off Collision`)
  (`PrimitiveComponent.SetCollisionEnabled` (`self.Capsule`) "NoCollision"))

(fn `UserConstructionScript`)