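; Sword weapon Blueprint for a combo combat system, built on a parent that it calls on BeginPlay.
; BeginPlay disables the capsule's collision, then sets the combat type and sword combo table before running the parent's setup.
; Capsule overlaps pass the other actor to SendDamage as the hit path.
; Select and deselect events only print debug strings for drawing and sheathing.
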(event `self.OnSelected`
  (`KismetSystemLibrary.PrintString` "Sword"))

(event `self.OffSelected`
  (`KismetSystemLibrary.PrintString` "Sword Sheath"))

(event `self.ReceiveBeginPlay`
  (`PrimitiveComponent.SetCollisionEnabled` (`self.Capsule`) "NoCollision")
  (set `self.CombatType` "NewEnumerator1")
  (set `self.ComboTable` "/Game/Weapons/Combo/Sword_Combo_Table.Sword_Combo_Table")
  (`parent.ReceiveBeginPlay`) ; __super::BeginPlay
)

(event `self.Capsule.OnComponentBeginOverlap`
  (params (OverlappedComponent :type "PrimitiveComponent Object Reference") (OtherActor :type "Actor Object Reference") (OtherComp :type "PrimitiveComponent Object Reference") (OtherBodyIndex :type Integer) (bFromSweep :type Boolean) (SweepResult :type "HitResult Structure (by ref)"))
  (`self.SendDamage` OtherActor))

(fn `UserConstructionScript`)