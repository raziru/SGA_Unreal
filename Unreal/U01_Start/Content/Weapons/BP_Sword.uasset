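; BP_Sword is a melee weapon actor that damages Characters its capsule hitbox touches.
; The capsule's collision is disabled on BeginPlay, and this file contains no logic that re-enables it.
; On capsule overlap, it ignores its owner, casts the other actor to Character, and applies Power as damage, credited to the owner's instigator controller.
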(event `self.ReceiveBeginPlay`
  (`PrimitiveComponent.SetCollisionEnabled` (`self.Capsule`) "NoCollision"))

(event `self.Capsule.OnComponentBeginOverlap`
  (params (OverlappedComponent :type "PrimitiveComponent Object Reference") (OtherActor :type "Actor Object Reference") (OtherComp :type "PrimitiveComponent Object Reference") (OtherBodyIndex :type Integer) (bFromSweep :type Boolean) (SweepResult :type "HitResult Structure (by ref)"))
  (if (!= OtherActor (`self.GetOwner`))
    (bind _ascharacter (cast `Character` OtherActor))
    (`GameplayStatics.ApplyDamage` _ascharacter (`self.Power`) (`self.GetInstigatorController` (`self.GetOwner`)) self)))

(fn `UserConstructionScript`)