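; BP_IWeapon is a weapon interface, with stub functions that return only default values.
; It declares getter and setter pairs for weapon state, combat and can-move, the first two returning enums and the last a boolean.
; It also declares a WeaponChange call that takes a weapon and a getter for the current weapon, leaving all behavior to implementers.
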(fn `GetWeapon_CanMove`
  (returns (CanMove :type Boolean))
  (return false))

(fn `GetWeapon_Combat`
  (returns (Combat :type "/Game/Enums/ECombatStyle Enum"))
  (return "NewEnumerator0"))

(fn `GetWeapon_Current`
  (returns (NewParam :type Boolean))
  (return false))

(fn `GetWeapon_State`
  (returns (state :type "/Game/Enums/EStateType Enum"))
  (return "NewEnumerator0"))

(fn `SetWeapon_CanMove`
  (params (CanMove :type Boolean))
  (returns (Result :type Boolean))
  (return false))

(fn `SetWeapon_Combat`
  (params (Combat :type "/Game/Enums/ECombatStyle Enum" :default "NewEnumerator0"))
  (returns (Result :type "/Game/Enums/ECombatStyle Enum"))
  (return "NewEnumerator0"))

(fn `SetWeapon_State`
  (params (State :type "/Game/Enums/EStateType Enum" :default "NewEnumerator0"))
  (returns (Result :type "/Game/Enums/EStateType Enum"))
  (return "NewEnumerator0"))

(fn `WeaponChange`
  (params (Weapon :type "/Game/Weapon/BP_Weapon Object Reference"))
  (returns (Result :type "/Game/Weapon/BP_Weapon Object Reference"))
  (return null))