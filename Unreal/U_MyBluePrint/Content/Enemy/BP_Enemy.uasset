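; BP_Enemy is a melee enemy that spawns a sword on its hand socket and shows a name label and health bar.
; Tick triggers a weapon attack every three seconds unless Damaged is set.
; Damage lowers health, turns it toward the attacker and plays the player's combo effect, then either a hit reaction with knockback or a one-time death montage that destroys enemy and weapon.
; Weapon accessor functions are partly stubbed.
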(event `self.ReceiveBeginPlay`
  (`|ExecutionSequence`
    (:`then_0`
      (bind _returnvalue (`|SpawnActorFromClass` "/Game/Weapon/Combo/BP_Sword.BP_Sword_C" (`KismetMathLibrary.MakeTransform` (0.0 0.0 0.0)) "Undefined" "OverrideRootScale" self null))
      (bind _output_get (set `self.Weapon` _returnvalue))
      (`self.K2_AttachToComponent` _output_get (`self.Mesh`) "GreatSword_Socket" "KeepRelative" "KeepRelative" "KeepRelative" true)
      (set `self.State` "NewEnumerator0")
      (set `self.Combat` "NewEnumerator1"))
    (:`then_1`
      (`self.UpdateHealthBar`))
    (:`then_2`
      (`ActorComponent.SetActive` (`self.Effect`) false false))
    (:`then_3`
      (`TextRenderComponent.K2_SetText` (`self.TextRender`) (`KismetTextLibrary.Conv_StringToText` (`KismetSystemLibrary.GetDisplayName` self))))
    (:`then_4`
      (`SceneComponent.SetVisibility` (`self.Cursor`) false false))))

(event `self.ReceiveAnyDamage`
  (params (Damage :type "Float (single-precision)") (DamageType :type "DamageType Object Reference") (InstigatedBy :type "Controller Object Reference") (DamageCauser :type "Actor Object Reference"))
  (bind (_returnvalue_x _returnvalue_y) (`KismetMathLibrary.BreakVector` (`self.K2_GetActorLocation`)))
  (bind _effect (`self.Effect`))
  (bind (_returnvalue_x_2 _returnvalue_y_2) (`KismetMathLibrary.BreakVector` (`self.K2_GetActorLocation` (`self.Attacker`))))
  (set `self.Causer` DamageCauser)
  (bind _ascharacter (cast `Character` (`Controller.K2_GetPawn` InstigatedBy)))
  (set `self.Attacker` _ascharacter)
  (set `self.Damage` Damage)
  (set `/Game/Components/StatusComponet.CurHealth` (`KismetMathLibrary.FClamp` (- (`/Game/Components/StatusComponet.CurHealth` (`self.CharacterStatus`)) (`self.Damage`)) 0.0 (`/Game/Components/StatusComponet.MaxHeallth` (`self.CharacterStatus`))) (`self.CharacterStatus`))
  (`self.UpdateHealthBar`)
  (`self.K2_SetActorRotation` (`KismetMathLibrary.FindLookAtRotation` (`KismetMathLibrary.MakeVector` _returnvalue_x _returnvalue_y) (`KismetMathLibrary.MakeVector` _returnvalue_x_2 _returnvalue_y_2)))
  (bind _asbp_player (cast `/Game/Player/BP_Player` (`self.Attacker`)))
  (bind _asbp_combo (cast `/Game/Weapon/Combo/BP_Combo` (`self.Causer`)))
  (`/Game/Player/BP_Player.PlayLastComboEffect` _asbp_player self (`/Game/Weapon/Combo/BP_Combo.LastComboParticle` _asbp_combo))
  (if (<= (`/Game/Components/StatusComponet.CurHealth` (`self.CharacterStatus`)) 0.0)
    (`/Engine/EditorBlueprintResources/StandardMacros.DoOnce` false
      (:`Completed`
        (set `self.Dead` true)
        (`PrimitiveComponent.SetCollisionEnabled` (`self.CapsuleComponent`) "NoCollision")
        (bind _returnvalue (`self.PlayAnimMontage` "/Game/Character/Montages/GetHitBackFall_Montage.GetHitBackFall_Montage"))
        (`KismetSystemLibrary.Delay` (- _returnvalue 1.162))
        (`self.K2_DestroyActor`)
        (`self.K2_DestroyActor` (`self.Weapon`))))
    (else
      (`self.PlayAnimMontage` "/Game/Character/Montages/Hit_Reaction_Montage.Hit_Reaction_Montage" 2.0)
      (cast `/Game/Weapon/Combo/BP_Combo` (`self.Causer`))
      (`self.K2_AddActorWorldOffset` (* (`KismetMathLibrary.Vector_Normal2D` (`self.GetActorForwardVector`)) (* (`CharacterMovementComponent.Mass` (`self.CharacterMovement`)) -0.2)))
      (`ActorComponent.SetActive` (`self.Effect`) false false)
      (`ParticleSystemComponent.SetTemplate` _effect "/Game/Effects/P_AOE_Ice_CircleAttack.P_AOE_Ice_CircleAttack")
      (`KismetSystemLibrary.Delay` 3.0)
      (`ActorComponent.SetActive` _effect false false)
      (`/Game/Weapon/BP_Weapon.EndAttack` (`self.Weapon`)))))

(event `self.ReceiveTick`
  (params (DeltaSeconds :type "Float (single-precision)"))
  (if (`self.Damaged`)
    (set `self.Frequency` 0.0)
    (else
      (bind _output_get (set `self.Frequency` (+ DeltaSeconds (`self.Frequency`))))
      (if (>= _output_get 3.0)
        (`self.Attack`)
        (set `self.Frequency` 0.0)))))

(event `Attack`
  (bind _weapon (`self.Weapon`))
  (`/Engine/EditorBlueprintResources/StandardMacros.IsValid` _weapon
    (:`Is Valid`
      (`/Game/Weapon/BP_Weapon.Attack` _weapon))))

(fn `Get_Damaged`
  (returns (Result :type Boolean))
  (return false))

(fn `GetWeapon_CanMove`
  (returns (CanMove :type Boolean))
  (return (`self.Can Move`)))

(fn `GetWeapon_Combat`
  (returns (Combat :type "/Game/Enums/ECombatStyle Enum"))
  (return (`self.Combat`)))

(fn `GetWeapon_Current`
  (returns (Result :type "/Game/Weapon/BP_Weapon Object Reference"))
  (return (`self.Weapon`)))

(fn `GetWeapon_State`
  (returns (state :type "/Game/Enums/EStateType Enum"))
  (return (`self.State`)))

(fn `Set_Damaged`
  (params (Damaged :type Boolean))
  (returns (Result :type Boolean))
  (return false))

(fn `SetWeapon_CanMove`
  (params (CanMove :type Boolean))
  (returns (Result :type Boolean))
  (bind _output_get (set `self.Can Move` CanMove))
  (return _output_get))

(fn `SetWeapon_Combat`
  (params (Combat :type "/Game/Enums/ECombatStyle Enum" :default "NewEnumerator0"))
  (returns (Result :type "/Game/Enums/ECombatStyle Enum"))
  (bind _output_get (set `self.Combat` Combat))
  (return _output_get))

(fn `SetWeapon_State`
  (params (State :type "/Game/Enums/EStateType Enum" :default "NewEnumerator0"))
  (returns (Result :type "/Game/Enums/EStateType Enum"))
  (bind _output_get (set `self.State` State))
  (return _output_get))

(fn `UpdateHealthBar`
  (bind _characterstatus (`self.CharacterStatus`))
  (bind _aswb_health_bar (cast `/Game/Widgets/WB_HealthBar` (`WidgetComponent.GetUserWidgetObject` (`self.HealthBar`))))
  (`/Game/Widgets/WB_HealthBar.UpdateHealthBar` _aswb_health_bar (`/Game/Components/StatusComponet.CurHealth` _characterstatus) (`/Game/Components/StatusComponet.MaxHeallth` _characterstatus)))

(fn `UserConstructionScript`)

(fn `Weapon_DecreaseHealth`
  (params (Health :type "Float (double-precision)"))
  (returns (Result :type "Float (double-precision)"))
  (return 0.0))

(fn `Weapon_IncreaseHealth`
  (params (Health :type "Float (double-precision)"))
  (returns (Result :type "Float (double-precision)"))
  (return 0.0))

(fn `WeaponChange`
  (params (`New Weapon` :type "/Game/Weapon/BP_Weapon Object Reference"))
  (returns (Result :type "/Game/Weapon/BP_Weapon Object Reference"))
  (bind _new_weapon (`local.New Weapon`))
  (if (!= `New Weapon` (`self.Weapon`))
    (`/Engine/EditorBlueprintResources/StandardMacros.IsValid` (`self.Weapon`)
      (:`Is Valid`
        (`/Game/Weapon/BP_Weapon.Off Selected` (`self.Weapon`)))
      (:`Is Not Valid`
        _))
    (`/Engine/EditorBlueprintResources/StandardMacros.IsValid` _new_weapon
      (:`Is Valid`
        (bind _output_get (set `self.Weapon` _new_weapon))
        (`/Game/Weapon/BP_Weapon.On Selected` _output_get)
        (return _output_get))
      (:`Is Not Valid`
        (bind _output_get_2 (set `self.Weapon` null))
        (return _output_get_2)))))