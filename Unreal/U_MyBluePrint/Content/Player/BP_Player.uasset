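; Player character Blueprint for third-person sword combat with walk, jump, roll, backstep and health bar.
; A State enum gates actions; draw and sheath toggle strafe-style rotation, with interface callbacks moving the spawned sword between sockets.
; Attack inputs delegate to the current weapon.
; Lock-on sphere-traces enemies, picks one by camera dot product, steers control rotation on Tick and switches sideways; the damage, hit-reaction and death chain is unconnected from AnyDamage.
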(fn `CanSwordAttack`
  (returns (CanAttack :type Boolean))
  (return (and (`|EnumEquality` (`self.State`) "NewEnumerator0") (`|EnumEquality` (`self.Combat`) "NewEnumerator1"))))

(fn `Get_Damaged`
  (returns (Result :type Boolean))
  (return (`self.Damaged`)))

(fn `GetLastCombo`
  (returns (LastCombo :type Boolean))
  (bind _asbp_combo (cast `/Game/Weapon/Combo/BP_Combo` (`self.Weapon`)))
  (return (`/Game/Weapon/Combo/BP_Combo.LastCombo` _asbp_combo)))

(fn `GetNearestEnemy`
  (params (`Is Right` :type Boolean))
  (locals (Map :type "Map of Float (double-precision) to /Game/Enemy/BP_Enemy Object Reference") (Minimum :type "Float (double-precision)" :default 100000.0) (MinimumEnemy :type "/Game/Enemy/BP_Enemy Object Reference") (Distance :type "Float (double-precision)"))
  (bind _returnvalue (`self.K2_GetActorRotation`))
  (bind _returnvalue_2 (`KismetMathLibrary.Abs` (`local.Distance`)))
  (`/Engine/EditorBlueprintResources/StandardMacros.IsValid` (`self.LookOnEnemy`)
    (:`Is Valid`
      (for _array_element (`self.TargetEnemies`)
        (`/Engine/EditorBlueprintResources/StandardMacros.IsValid` _array_element
          (:`Is Valid`
            (if (!= _array_element (`self.LookOnEnemy`))
              (`BlueprintMapLibrary.Map_Add` (`local.Map`) (`KismetMathLibrary.Dot_VectorVector` (`KismetMathLibrary.GetUpVector` _returnvalue) (`KismetMathLibrary.Cross_VectorVector` (`KismetMathLibrary.GetForwardVector` _returnvalue) (- (`self.K2_GetActorLocation` _array_element) (`self.K2_GetActorLocation`)))) _array_element)))))
      (bind _keys (`BlueprintMapLibrary.Map_Keys` (`local.Map`)))
      (for _array_element_2 _keys
        (set `local.Distance` _array_element_2)
        (if (`local.Is Right`)
          (if (> (`local.Distance`) 0.0)
            (if (>= (`local.Minimum`) _returnvalue_2) :!label _label
              (set `local.Minimum` _returnvalue_2)
              (set `local.MinimumEnemy` (`BlueprintMapLibrary.Map_Find` (`local.Map`) (`local.Distance`)))))
          (elif (< (`local.Distance`) 0.0)
            (goto _label))))
      (`self.SetTargetCursor` (`local.MinimumEnemy`))
      (set `self.LookOnEnemy` (`local.MinimumEnemy`)))))

(fn `GetRollDirection`
  (returns (ReturnValue :type "Rotator Structure"))
  (return (`KismetMathLibrary.FindLookAtRotation` (`self.K2_GetActorLocation`) (+ (`self.K2_GetActorLocation`) (`KismetMathLibrary.Vector_Normal2D` (`self.GetVelocity`))))))

(fn `GetStepDirection`
  (returns (ReturnValue :type "Rotator Structure"))
  (if (not (< 0.0 (`self.GetInputAxisValue`)))
    (return (`KismetMathLibrary.FindLookAtRotation` (+ (`self.K2_GetActorLocation`) (`KismetMathLibrary.Vector_Normal2D` (`self.GetVelocity`))) (`self.K2_GetActorLocation`)))))

(fn `GetTargetEnemy`
  (returns (Target :type "/Game/Enemy/BP_Enemy Object Reference"))
  (locals (Result :type "/Game/Enemy/BP_Enemy Object Reference") (Angle :type "Float (double-precision)" :default -2.0))
  (for _array_element (`self.TargetEnemies`)
    (bind _returnvalue (`self.GetDotProductTo` _array_element (`GameplayStatics.GetPlayerCameraManager` 0)))
    (if (>= _returnvalue (`local.Angle`))
      (set `local.Angle` _returnvalue)
      (set `local.Result` _array_element)))
  (`self.SetTargetCursor` (`local.Result`))
  (return (`local.Result`)))

(fn `GetTraceTargets`
  (bind _returnvalue (`self.K2_GetActorLocation`))
  (bind _outhits (`KismetSystemLibrary.SphereTraceMultiForObjects` :`Start` _returnvalue :`End` (+ _returnvalue (`self.LookDistance`)) :`Radius` (`self.LookDistance`) :`ObjectTypes` (`|MakeArray` "ObjectTypeQuery3" :!type "EObjectTypeQuery Enum") :`DrawDebugType` "ForDuration" :`TraceColor` (struct :`G` 1.0 :`A` 1.0) :`TraceHitColor` (struct :`R` 1.0 :`A` 1.0) :`DrawTime` 2.0))
  (for _array_element _outhits
    (bind _asbp_enemy (cast `/Game/Enemy/BP_Enemy` (`.HitActor` (`GameplayStatics.BreakHitResult` _array_element))))
    (`KismetArrayLibrary.Array_AddUnique` (`self.TargetEnemies`) _asbp_enemy)))

(fn `GetWeapon_CanMove`
  (returns (CanMove :type Boolean))
  (return (`self.CanMove`)))

(fn `GetWeapon_Combat`
  (returns (Combat :type "/Game/Enums/ECombatStyle Enum"))
  (return (`self.Combat`)))

(fn `GetWeapon_Current`
  (returns (Result :type "/Game/Weapon/BP_Weapon Object Reference"))
  (return (`self.Weapon`)))

(fn `GetWeapon_State`
  (returns (state :type "/Game/Enums/EStateType Enum"))
  (return (`self.State`)))

(fn `Set_Damaged`
  (params (Damaged :type Boolean))
  (returns (Result :type Boolean))
  (bind _output_get (set `self.Damaged` Damaged))
  (return _output_get))

(fn `SetLastCombo`
  (params (`Last Combo` :type Boolean))
  (returns (Result :type Boolean))
  (bind _asbp_combo (cast `/Game/Weapon/Combo/BP_Combo` (`self.Weapon`)))
  (bind _output_get (set `/Game/Weapon/Combo/BP_Combo.LastCombo` `Last Combo` _asbp_combo))
  (return _output_get))

(fn `SetTargetCursor`
  (params (Enemy :type "/Game/Enemy/BP_Enemy Object Reference"))
  (`/Engine/EditorBlueprintResources/StandardMacros.IsValid` Enemy
    (:`Is Valid`
      (for _array_element (`self.TargetEnemies`)
        (`/Engine/EditorBlueprintResources/StandardMacros.IsValid` _array_element
          (:`Is Valid`
            (if (== _array_element (`local.Enemy`))
              (bind _cursor (`/Game/Enemy/BP_Enemy.Cursor` _array_element))
              (`SceneComponent.SetVisibility` _cursor true false)
              (else
                (`SceneComponent.SetVisibility` _cursor false false)))))))
    (:`Is Not Valid`
      (for _array_element_2 (`self.TargetEnemies`)
        (`/Engine/EditorBlueprintResources/StandardMacros.IsValid` _array_element_2
          (:`Is Valid`
            (`SceneComponent.SetVisibility` (`/Game/Enemy/BP_Enemy.Cursor` _array_element_2) false false)))))))

(fn `SetWeapon_CanMove`
  (params (CanMove :type Boolean))
  (returns (Result :type Boolean))
  (bind _output_get (set `self.CanMove` CanMove))
  (return _output_get))

(fn `SetWeapon_Combat`
  (params (Combat :type "/Game/Enums/ECombatStyle Enum" :default "NewEnumerator0"))
  (returns (Result :type "/Game/Enums/ECombatStyle Enum"))
  (bind _output_get (set `self.Combat` Combat))
  (return _output_get))

(fn `SetWeapon_State`
  (params (State :type "/Game/Enums/EStateType Enum" :default "NewEnumerator0"))
  (returns (Result :type "/Game/Enums/EStateType Enum"))
  (bind _output_get (set `self.State` State))
  (return _output_get))

(fn `UpdateHealthBar`
  (bind _characterstatus (`self.CharacterStatus`))
  (bind _aswb_health_bar (cast `/Game/Widgets/WB_HealthBar` (`WidgetComponent.GetUserWidgetObject` (`self.HealthBar`))))
  (`/Game/Widgets/WB_HealthBar.UpdateHealthBar` _aswb_health_bar (`/Game/Components/StatusComponet.CurHealth` _characterstatus) (`/Game/Components/StatusComponet.MaxHeallth` _characterstatus)))

(fn `UserConstructionScript`)

(fn `Weapon_DecreaseHealth`
  (params (Health :type "Float (double-precision)"))
  (returns (Result :type "Float (double-precision)"))
  (return 0.0))

(fn `Weapon_Equipped`
  (returns (Result :type Boolean))
  (`self.Equipped`)
  (return false))

(fn `Weapon_GrabSword`
  (returns (Result :type Boolean))
  (`self.Grab Sword`)
  (return false))

(fn `Weapon_IncreaseHealth`
  (params (Health :type "Float (double-precision)"))
  (returns (Result :type "Float (double-precision)"))
  (return 0.0))

(fn `Weapon_UnEquipped`
  (returns (Result :type Boolean))
  (`self.UnEquipped`)
  (return false))

(fn `Weapon_UnGrabSword`
  (returns (Result :type Boolean))
  (`self.UnGrabSword`)
  (return false))

(fn `WeaponChange`
  (params (`New Weapon` :type "/Game/Weapon/BP_Weapon Object Reference"))
  (returns (Result :type "/Game/Weapon/BP_Weapon Object Reference"))
  (bind _new_weapon (`local.New Weapon`))
  (if (!= `New Weapon` (`self.Weapon`))
    (`/Engine/EditorBlueprintResources/StandardMacros.IsValid` (`self.Weapon`)
      (:`Is Valid`
        (`/Game/Weapon/BP_Weapon.Off Selected` (`self.Weapon`)))
      (:`Is Not Valid`
        _))
    (`/Engine/EditorBlueprintResources/StandardMacros.IsValid` _new_weapon
      (:`Is Valid`
        (bind _output_get (set `self.Weapon` _new_weapon))
        (`/Game/Weapon/BP_Weapon.On Selected` _output_get)
        (return _output_get))
      (:`Is Not Valid`
        (bind _output_get_2 (set `self.Weapon` null))
        (return _output_get_2)))))