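; Shoe item that changes the owning player's walk speed while it is in use.
; BeginPlay caches the owner's default MaxWalkSpeed from its CharacterMovement component.
; Use calls the parent logic and applies ItemWalkSpeed, while EndUse calls the parent and restores the cached speed, both printing the resulting value.
; The selection and deselection events are empty.
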(event `self.ReceiveBeginPlay`
  (set `self.DefaultWalkSpeed` (`CharacterMovementComponent.MaxWalkSpeed` (`Character.CharacterMovement` (`self.GetOwnerToPlayer`)))))

(event `self.Use`
  (`parent.Use`)
  (bind _output_get (set `CharacterMovementComponent.MaxWalkSpeed` (`self.ItemWalkSpeed`) (`Character.CharacterMovement` (`self.GetOwnerToPlayer`))))
  (`KismetSystemLibrary.PrintString` (`KismetStringLibrary.Conv_DoubleToString` _output_get)))

(event `self.EndUse`
  (`parent.EndUse`)
  (bind _output_get (set `CharacterMovementComponent.MaxWalkSpeed` (`self.DefaultWalkSpeed`) (`Character.CharacterMovement` (`self.GetOwnerToPlayer`))))
  (`KismetSystemLibrary.PrintString` (`KismetStringLibrary.Conv_DoubleToString` _output_get)))

(event `self.On Selected`)

(event `self.Off Selected`)

(fn `UserConstructionScript`
  (`parent.UserConstructionScript`))