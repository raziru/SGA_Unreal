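; Shoes item that changes the owning player's walk speed while in use and shows a shoe on each foot when equipped.
; Use caches the current MaxWalkSpeed before applying ItemWalkSpeed, and EndUse restores it, both printing the result.
; Equip spawns left and right shoe actors on the mesh's foot sockets without calling the parent version.
; UnEquip only hides their meshes, so each Equip spawns a new pair.
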(event `self.ReceiveBeginPlay`)

(event `self.Use`
  (`parent.Use`)
  (set `self.DefaultWalkSpeed` (`CharacterMovementComponent.MaxWalkSpeed` (`Character.CharacterMovement` (`self.GetOwnerToPlayer`))))
  (bind _output_get (set `CharacterMovementComponent.MaxWalkSpeed` (`self.ItemWalkSpeed`) (`Character.CharacterMovement` (`self.GetOwnerToPlayer`))))
  (`KismetSystemLibrary.PrintString` (`KismetStringLibrary.Conv_DoubleToString` _output_get)))

(event `self.EndUse`
  (`parent.EndUse`)
  (bind _output_get (set `CharacterMovementComponent.MaxWalkSpeed` (`self.DefaultWalkSpeed`) (`Character.CharacterMovement` (`self.GetOwnerToPlayer`))))
  (`KismetSystemLibrary.PrintString` (`KismetStringLibrary.Conv_DoubleToString` _output_get)))

(event `self.On Selected`)

(event `self.Off Selected`)

(fn `Equip`
  (`KismetSystemLibrary.PrintString` (`KismetSystemLibrary.GetDisplayName` self))
  (`|ExecutionSequence`
    (:`then_0`
      (bind _returnvalue (`|SpawnActorFromClass` "/Game/Items/BP_Item_Shoes_Right.BP_Item_Shoes_Right_C" (`KismetMathLibrary.MakeTransform` (0.0 0.0 0.0)) "Undefined" "OverrideRootScale" self null))
      (bind _output_get (set `self.Shoes_Right` _returnvalue))
      (`self.K2_AttachToComponent` _output_get (`Character.Mesh` (`self.GetOwnerToPlayer`)) "Right_Foot" "KeepRelative" "KeepRelative" "KeepRelative" true))
    (:`then_1`
      (bind _returnvalue_2 (`|SpawnActorFromClass` "/Game/Items/BP_Item_Shoes_Left.BP_Item_Shoes_Left_C" (`KismetMathLibrary.MakeTransform` (0.0 0.0 0.0)) "Undefined" "OverrideRootScale" self null))
      (bind _output_get_2 (set `self.Shoes_Left` _returnvalue_2))
      (`self.K2_AttachToComponent` _output_get_2 (`Character.Mesh` (`self.GetOwnerToPlayer`)) "Left_Foot" "KeepRelative" "KeepRelative" "KeepRelative" true))
    (:`then_2`
      (`SceneComponent.SetVisibility` (`/Game/Items/BP_Item_Shoes_Left.StaticMesh` (`self.Shoes_Left`)) true false)
      (`SceneComponent.SetVisibility` (`/Game/Items/BP_Item_Shoes_Right.StaticMesh` (`self.Shoes_Right`)) true false))))

(fn `UnEquip`
  (`/Engine/EditorBlueprintResources/StandardMacros.IsValid` (`self.Shoes_Left`)
    (:`Is Valid`
      (`SceneComponent.SetVisibility` (`/Game/Items/BP_Item_Shoes_Left.StaticMesh` (`self.Shoes_Left`)) false false)
      (`SceneComponent.SetVisibility` (`/Game/Items/BP_Item_Shoes_Right.StaticMesh` (`self.Shoes_Right`)) false false))))

(fn `UserConstructionScript`
  (`parent.UserConstructionScript`))