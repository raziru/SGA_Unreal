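; BP_Item_Lantern is a lantern item that lights up the player while it is in use.
; Its Use and EndUse overrides call the parent logic, then show or hide the owning player's SpotLight component.
; The light lives on the player rather than on the item, and the construction script only calls its parent.
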(event `self.Use`
  (`parent.Use`)
  (`SceneComponent.SetVisibility` (`/Game/Player/BP_Player.SpotLight` (`self.GetOwnerToPlayer`)) true false))

(event `self.EndUse`
  (`parent.EndUse`)
  (`SceneComponent.SetVisibility` (`/Game/Player/BP_Player.SpotLight` (`self.GetOwnerToPlayer`)) false false))

(fn `UserConstructionScript`
  (`parent.UserConstructionScript`))