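; BP_Item is a pickup item that looks like a base class, with mostly empty functions for effects, type, health, equipping and selection.
; On Interact it passes its ItemInfo to the first player's BP_Player through PickUp, then destroys itself.
; Use and EndUse toggle an IsActive flag, and GetOwnerToPlayer returns the owner cast to BP_Player.
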(event `On Selected`)

(event `Off Selected`)

(event `/Game/BP_Interact.Interact`
  (bind _asbp_player (cast `/Game/Player/BP_Player` (`GameplayStatics.GetPlayerCharacter` 0)))
  (`/Game/Player/BP_Player.PickUp` _asbp_player (`self.ItemInfo`))
  (`self.K2_DestroyActor`))

(fn `DecreasHealth`)

(fn `EndEffect`)

(fn `EndEquip`)

(fn `EndUnEquip`)

(fn `EndUse`
  (set `self.isActive` false))

(fn `Equip`)

(fn `GetEffect`)

(fn `GetOwnerToPlayer`
  (returns (`AsBP Player` :type "/Game/Player/BP_Player Object Reference"))
  (bind _asbp_player (cast `/Game/Player/BP_Player` (`self.GetOwner`)))
  (return _asbp_player))

(fn `GetType`)

(fn `IncreaseHealth`)

(fn `SetEffect`)

(fn `UnEquip`)

(fn `Use`
  (set `self.isActive` true))

(fn `UserConstructionScript`)