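; BP_Weapon is a base weapon Blueprint with empty hooks for selection, attack, end attack and special attack.
; It reads and changes the owner's movement, combat, state and health through BP_IWeapon messages, mostly after an interface check.
; CanAttack requires a specific owner state and a combat mode matching the weapon's CombatStyle.
; SendDamage applies Power as damage to Characters other than the owner, crediting the owner's instigator controller.
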(event `On Selected`)

(event `Off Selected`)

(fn `Attack`)

(fn `CanAttack`
  (returns (Result :type Boolean))
  (return (and (`|EnumEquality` (`self.GetState`) "NewEnumerator0") (`|EnumEquality` (`self.GetCombat`) (`self.CombatStyle`)))))

(fn `DecreaseHealth`
  (params (Health :type "Float (double-precision)"))
  (returns (Result :type "Float (double-precision)"))
  (bind _returnvalue (`self.GetOwner`))
  (if (`KismetSystemLibrary.DoesImplementInterface` _returnvalue "/Game/BP_IWeapon.BP_IWeapon_C")
    (bind _result (message `/Game/BP_IWeapon.Weapon_DecreaseHealth` _returnvalue Health))
    (return _result)))

(fn `EndAttack`)

(fn `GetCanMove`
  (returns (CanMove :type Boolean))
  (bind _canmove (message `/Game/BP_IWeapon.GetWeapon_CanMove` (`self.GetOwner`)))
  (return _canmove))

(fn `GetCombat`
  (returns (Combat :type "/Game/Enums/ECombatStyle Enum"))
  (bind _returnvalue (`self.GetOwner`))
  (if (`KismetSystemLibrary.DoesImplementInterface` _returnvalue "/Game/BP_IWeapon.BP_IWeapon_C")
    (bind _combat (message `/Game/BP_IWeapon.GetWeapon_Combat` _returnvalue))
    (return _combat)))

(fn `GetState`
  (returns (state :type "/Game/Enums/EStateType Enum"))
  (bind _returnvalue (`self.GetOwner`))
  (if (`KismetSystemLibrary.DoesImplementInterface` _returnvalue "/Game/BP_IWeapon.BP_IWeapon_C")
    (bind _state (message `/Game/BP_IWeapon.GetWeapon_State` _returnvalue))
    (return _state)))

(fn `IncreaseHealth`
  (params (Health :type "Float (double-precision)"))
  (returns (Result :type "Float (double-precision)"))
  (bind _returnvalue (`self.GetOwner`))
  (if (`KismetSystemLibrary.DoesImplementInterface` _returnvalue "/Game/BP_IWeapon.BP_IWeapon_C")
    (bind _result (message `/Game/BP_IWeapon.Weapon_IncreaseHealth` _returnvalue Health))
    (return _result)))

(fn `SendDamage`
  (params (OtherActor :type "Actor Object Reference"))
  (returns (Result :type Boolean))
  (if (!= OtherActor (`self.GetOwner`))
    (bind _ascharacter (cast `Character` OtherActor)
      (:`then`
        (bind _returnvalue (`GameplayStatics.ApplyDamage` _ascharacter (`self.power`) (`self.GetInstigatorController` (`self.GetOwner`)) self))
        (`KismetSystemLibrary.PrintString` (`KismetStringLibrary.Conv_DoubleToString` _returnvalue))
        (return true))
      (:`CastFailed`
        (return false)))
    (else
      (return false))))

(fn `SetCanMove`
  (params (CanMove :type Boolean))
  (returns (Result :type Boolean))
  (bind _returnvalue (`self.GetOwner`))
  (if (`KismetSystemLibrary.DoesImplementInterface` _returnvalue "/Game/BP_IWeapon.BP_IWeapon_C")
    (bind _result (message `/Game/BP_IWeapon.SetWeapon_CanMove` _returnvalue CanMove))
    (return _result)))

(fn `SetCombat`
  (params (Combat :type "/Game/Enums/ECombatStyle Enum" :default "NewEnumerator0"))
  (returns (NewCombat :type "/Game/Enums/ECombatStyle Enum"))
  (bind _returnvalue (`self.GetOwner`))
  (if (`KismetSystemLibrary.DoesImplementInterface` _returnvalue "/Game/BP_IWeapon.BP_IWeapon_C")
    (bind _result (message `/Game/BP_IWeapon.SetWeapon_Combat` _returnvalue Combat))
    (return _result)))

(fn `SetState`
  (params (state :type "/Game/Enums/EStateType Enum" :default "NewEnumerator0"))
  (returns (Result :type "/Game/Enums/EStateType Enum"))
  (bind _result (message `/Game/BP_IWeapon.SetWeapon_State` (`self.GetOwner`) state))
  (return _result))

(fn `Special Attack`)

(fn `UserConstructionScript`)