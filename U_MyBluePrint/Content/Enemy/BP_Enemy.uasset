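; BP_Enemy is an enemy character with a name label, a health bar and weapon state accessors.
; Damage lowers health, turns it toward the attacker and plays the player's combo effect, then triggers death or a hit reaction with mass-scaled knockback.
; Death and hit reactions follow only when BP_Player and BP_Combo casts succeed.
; Sword spawning is never run, and the ice hit effect is set but never activated.
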(event `self.ReceiveBeginPlay`
  (`|ExecutionSequence`
    (:`then_0`
      (set `self.CanDamaged` (`/Game/Components/StatusComponet.CanDamaged` (`self.CharacterStatus`))))
    (:`then_1`
      (`self.UpdateHealthBar`))
    (:`then_2`
      (`ActorComponent.SetActive` (`self.Effect`) false false))
    (:`then_4`
      (`SceneComponent.SetVisibility` (`self.Cursor`) false false))))

(event `self.ReceiveAnyDamage`
  (params (Damage :type "Float (single-precision)") (DamageType :type "DamageType Object Reference") (InstigatedBy :type "Controller Object Reference") (DamageCauser :type "Actor Object Reference"))
  (bind (_returnvalue_x _returnvalue_y) (`KismetMathLibrary.BreakVector` (`self.K2_GetActorLocation`)))
  (bind _effect (`self.Effect`))
  (bind (_returnvalue_x_2 _returnvalue_y_2) (`KismetMathLibrary.BreakVector` (`self.K2_GetActorLocation` (`self.Attacker`))))
  (if true
    (set `self.Causer` DamageCauser)
    (bind _ascharacter (cast `Character` (`Controller.K2_GetPawn` InstigatedBy)))
    (set `self.Attacker` _ascharacter)
    (set `self.Damage` Damage)
    (set `/Game/Components/StatusComponet.CurHealth` (`KismetMathLibrary.FClamp` (- (`/Game/Components/StatusComponet.CurHealth` (`self.CharacterStatus`)) (`self.Damage`)) 0.0 (`/Game/Components/StatusComponet.MaxHeallth` (`self.CharacterStatus`))) (`self.CharacterStatus`))
    (`self.UpdateHealthBar`)
    (`self.K2_SetActorRotation` (`KismetMathLibrary.FindLookAtRotation` (`KismetMathLibrary.MakeVector` _returnvalue_x _returnvalue_y) (`KismetMathLibrary.MakeVector` _returnvalue_x_2 _returnvalue_y_2)))
    (bind _asbp_player (cast `/Game/Player/BP_Player` (`self.Attacker`)))
    (bind _asbp_combo (cast `/Game/Weapon/Combo/BP_Combo` (`self.Causer`)))
    (`/Game/Player/BP_Player.PlayLastComboEffect` _asbp_player self (`/Game/Weapon/Combo/BP_Combo.LastComboParticle` _asbp_combo))
    (if (<= (`/Game/Components/StatusComponet.CurHealth` (`self.CharacterStatus`)) 0.0)
      (`/Engine/EditorBlueprintResources/StandardMacros.DoOnce` false
        (:`Completed`
          (set `self.Dead` true)
          (`PrimitiveComponent.SetCollisionEnabled` (`self.CapsuleComponent`) "NoCollision")
          (`self.PlayAnimMontage` "/Game/Character/Montages/GetHitBackFall_Montage.GetHitBackFall_Montage")))
      (else
        (`self.PlayAnimMontage` "/Game/Character/Montages/Hit_Reaction_Enemy_Montage.Hit_Reaction_Enemy_Montage" 2.0)
        (cast `/Game/Weapon/Combo/BP_Combo` (`self.Causer`))
        (`self.K2_AddActorWorldOffset` (* (`KismetMathLibrary.Vector_Normal2D` (`self.GetActorForwardVector`)) (* (`CharacterMovementComponent.Mass` (`self.CharacterMovement`)) -0.2)))
        (`ActorComponent.SetActive` (`self.Effect`) false false)
        (`ParticleSystemComponent.SetTemplate` _effect "/Game/Effects/P_AOE_Ice_CircleAttack.P_AOE_Ice_CircleAttack")
        (`KismetSystemLibrary.Delay` 3.0)
        (`ActorComponent.SetActive` _effect false false)))))

(event `self.ReceiveTick`
  (params (DeltaSeconds :type "Float (single-precision)")))

(event `Attack`
  (bind _weapon (`self.Weapon`))
  (`/Engine/EditorBlueprintResources/StandardMacros.IsValid` _weapon
    (:`Is Valid`
      (`/Game/Weapon/BP_Weapon.Attack` _weapon))))

(fn `Equipped`
  (set `self.State` "NewEnumerator0"))

(fn `Get_CanDamaged`
  (returns (Result :type Boolean))
  (return (`self.CanDamaged`)))

(fn `GetWeapon_CanMove`
  (returns (CanMove :type Boolean))
  (return (`self.Can Move`)))

(fn `GetWeapon_Combat`
  (returns (Combat :type "/Game/Enums/ECombatStyle Enum"))
  (return (`self.Combat`)))

(fn `GetWeapon_Current`
  (returns (Result :type "/Game/Weapon/BP_Weapon Object Reference"))
  (return (`self.Weapon`)))

(fn `GetWeapon_State`
  (returns (state :type "/Game/Enums/EStateType Enum"))
  (return (`self.State`)))

(fn `GrabSword`)

(fn `SelfDestory`
  (`self.K2_DestroyActor`)
  (bind _greatsword (`self.GreatSword`)
    (:`then`
      (`self.K2_DestroyActor` _greatsword))
    (:`else`)))

(fn `Set_CanDamaged`
  (params (Damaged :type Boolean))
  (returns (Result :type Boolean))
  (bind _output_get (set `self.CanDamaged` Damaged))
  (return _output_get))

(fn `SetWeapon_CanMove`
  (params (CanMove :type Boolean))
  (returns (Result :type Boolean))
  (bind _output_get (set `self.Can Move` CanMove))
  (return _output_get))

(fn `SetWeapon_Combat`
  (params (Combat :type "/Game/Enums/ECombatStyle Enum" :default "NewEnumerator0"))
  (returns (Result :type "/Game/Enums/ECombatStyle Enum"))
  (bind _output_get (set `self.Combat` Combat))
  (return _output_get))

(fn `SetWeapon_State`
  (params (State :type "/Game/Enums/EStateType Enum" :default "NewEnumerator0"))
  (returns (Result :type "/Game/Enums/EStateType Enum"))
  (bind _output_get (set `self.State` State))
  (return _output_get))

(fn `UnEquipped`
  (set `self.State` "NewEnumerator0"))

(fn `UnGrabSword`)

(fn `UpdateHealthBar`
  (bind _characterstatus (`self.CharacterStatus`))
  (bind _aswb_health_bar (cast `/Game/Widgets/WB_HealthBar` (`WidgetComponent.GetUserWidgetObject` (`self.HealthBar`))))
  (`/Game/Widgets/WB_HealthBar.UpdateHealthBar` _aswb_health_bar (`/Game/Components/StatusComponet.CurHealth` _characterstatus) (`/Game/Components/StatusComponet.MaxHeallth` _characterstatus)))

(fn `UserConstructionScript`
  (`TextRenderComponent.K2_SetText` (`self.TextRender`) (`KismetTextLibrary.Conv_StringToText` (`KismetSystemLibrary.GetDisplayName` self))))

(fn `Weapon_Dead`
  (returns (Result :type Boolean))
  (`self.SelfDestory`)
  (return false))

(fn `Weapon_DecreaseHealth`
  (params (Health :type "Float (double-precision)"))
  (returns (Result :type "Float (double-precision)"))
  (return 0.0))

(fn `Weapon_Equipped`
  (returns (Result :type Boolean))
  (`self.Equipped`)
  (return false))

(fn `Weapon_GrabSword`
  (returns (Result :type Boolean))
  (`self.GrabSword`)
  (return false))

(fn `Weapon_Hitted`
  (returns (Result :type Boolean))
  (set `self.State` "NewEnumerator0")
  (return false))

(fn `Weapon_IncreaseHealth`
  (params (Health :type "Float (double-precision)"))
  (returns (Result :type "Float (double-precision)"))
  (return 0.0))

(fn `Weapon_UnEquipped`
  (returns (Result :type Boolean))
  (`self.UnEquipped`)
  (return false))

(fn `Weapon_UnGrabSword`
  (returns (Result :type Boolean))
  (`self.UnGrabSword`)
  (return false))

(fn `WeaponChange`
  (params (`New Weapon` :type "/Game/Weapon/BP_Weapon Object Reference"))
  (returns (Result :type "/Game/Weapon/BP_Weapon Object Reference"))
  (bind _new_weapon (`local.New Weapon`))
  (if (!= `New Weapon` (`self.Weapon`))
    (`/Engine/EditorBlueprintResources/StandardMacros.IsValid` (`self.Weapon`)
      (:`Is Valid`
        (`/Game/Weapon/BP_Weapon.Off Selected` (`self.Weapon`)))
      (:`Is Not Valid`
        _))
    (`/Engine/EditorBlueprintResources/StandardMacros.IsValid` _new_weapon
      (:`Is Valid`
        (bind _output_get (set `self.Weapon` _new_weapon))
        (`/Game/Weapon/BP_Weapon.On Selected` _output_get)
        (return _output_get))
      (:`Is Not Valid`
        (bind _output_get_2 (set `self.Weapon` null))
        (return _output_get_2)))))