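; Sword-wielding enemy AI Blueprint that adds a greatsword to its parent class's equip behavior.
; On BeginPlay it spawns a BP_GreatSword owned by itself and attaches it to the holster socket on the mesh.
; GrabSword and UnGrabSword move the sword between hand and holster sockets.
; Equipped and UnEquipped extend the parent events, calling WeaponChange to set or clear the weapon and switching the Combat state.
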(event `self.GrabSword`
  (`self.K2_AttachToComponent` (`self.GreatSword`) (`self.Mesh`) "GreatSword_Socket" "KeepRelative" "KeepRelative" "KeepRelative" true))

(event `self.Equipped`
  (`parent.Equipped`)
  (`self.WeaponChange` (`self.GreatSword`))
  (set `self.Combat` "NewEnumerator1"))

(event `self.UnEquipped`
  (`parent.UnEquipped`)
  (`self.WeaponChange` null)
  (set `self.Combat` "NewEnumerator0"))

(event `self.UnGrabSword`
  (`self.K2_AttachToComponent` (`self.GreatSword`) (`self.Mesh`) "Holster_GreatSword" "KeepRelative" "KeepRelative" "KeepRelative" true))

(event `self.ReceiveBeginPlay`
  (`parent.ReceiveBeginPlay`)
  (bind _returnvalue (`|SpawnActorFromClass` "/Game/Weapon/Combo/BP_GreatSword.BP_GreatSword_C" (`KismetMathLibrary.MakeTransform` (0.0 0.0 0.0)) "Undefined" "OverrideRootScale" self null))
  (bind _output_get (set `self.GreatSword` _returnvalue))
  (`self.K2_AttachToComponent` _output_get (`self.Mesh`) "Holster_GreatSword" "KeepRelative" "KeepRelative" "KeepRelative" true))

(fn `UserConstructionScript`
  (`parent.UserConstructionScript`))