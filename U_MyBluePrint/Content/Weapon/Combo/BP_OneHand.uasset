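; BP_OneHand is a one-handed weapon that pairs its parent weapon behavior with a shield.
; On BeginPlay it spawns a BP_Item_Shield and attaches it to the mesh's holster socket.
; Grab and UnGrab move the shield between its hand and holster sockets, while right-click press and release start and end its use.
; Deselecting the weapon destroys the shield.
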(event `self.ReceiveBeginPlay`
  (`parent.ReceiveBeginPlay`)
  (bind _returnvalue (`|SpawnActorFromClass` "/Game/Items/BP_Item_Shield.BP_Item_Shield_C" (`KismetMathLibrary.MakeTransform` (0.0 0.0 0.0)) "Undefined" "OverrideRootScale" (`self.GetOwner`) null))
  (bind _output_get (set `self.Shield` _returnvalue))
  (`self.K2_AttachToComponent` _output_get (`self.Get Mesh`) (`/Game/Items/BP_Item.Holster` _output_get) "KeepRelative" "KeepRelative" "KeepRelative" true))

(event `self.Grab`
  (bind _shield (`self.Shield`))
  (`parent.Grab`)
  (`self.K2_AttachToComponent` _shield (`self.Get Mesh`) (`/Game/Items/BP_Item.Socket` _shield) "KeepRelative" "KeepRelative" "KeepRelative" true))

(event `self.UnGrab`
  (bind _shield (`self.Shield`))
  (`parent.UnGrab`)
  (`self.K2_AttachToComponent` _shield (`self.Get Mesh`) (`/Game/Items/BP_Item.Holster` _shield) "KeepRelative" "KeepRelative" "KeepRelative" true))

(event `self.RightClick`
  (`/Game/Items/BP_Item.Use` (`self.Shield`)))

(event `self.RightClickRelease`
  (`/Game/Items/BP_Item.EndUse` (`self.Shield`)))

(event `self.Off Selected`
  (`parent.Off Selected`)
  (`self.K2_DestroyActor` (`self.Shield`)))

(fn `UserConstructionScript`
  (`parent.UserConstructionScript`))