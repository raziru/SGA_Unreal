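; BP_Combo is a player melee weapon that picks a combo, jump or spin attack based on input and whether the owner is falling.
; BeginPlay loads combo montages from a data table, and attacks pressed during the combo window queue the next montage until EndAttack resets the chain.
; PowerComponent supplies per-step power, each character is damaged once until collision switches off, and sword sounds cycle through three cues.
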(event `self.ReceiveBeginPlay`
  (bind _outrownames (`DataTableFunctionLibrary.GetDataTableRowNames` (`self.ComboTable`)))
  (for _array_element _outrownames
    (bind _returnvalue (`|GetDataTableRow` (`self.ComboTable`) _array_element)
      (:`then`
        (`KismetArrayLibrary.Array_Add` (`self.ComboMontages`) _returnvalue)))))

(event `self.EndAttack`
  (`parent.EndAttack`)
  (`self.SetCanMove` true)
  (set `self.ComboCount` 0)
  (set `self.ExistNextCombo` false)
  (set `self.LastCombo` false)
  (`/Game/Components/PowerComponent.EndComboAttack` (`self.PowerComponent`))
  (set `self.SwordSoundIndex` 0))

(event `OnCollsioin`)

(event `OffCollsion`
  (`KismetArrayLibrary.Array_Clear` (`self.HittedCharacter`)))

(event `self.Attack`
  ;[1 1 1] Attack
  (if (`self.IsFalling`)
    (`self.Jump Attack`)
    (else
      (`self.ComboAttack`))))

(event `self.Special Attack`
  ;[1 1 1] Attack
  (if (not (`self.IsFalling`))
    (`self.SpinAttack`)))

(event `ComboAttack`
  ;[1 1 1] ComboAttack
  (if (`self.EnableNextCombo`)
    (`/Engine/EditorBlueprintResources/StandardMacros.IncrementInt` (`self.ComboCount`)
      (:`  `
        (set `self.EnableNextCombo` false)
        (set `self.ExistNextCombo` true)))
    (elif (`self.CanAttack`)
      (`self.SetState` "NewEnumerator1")
      (`self.PlayComboMontage`)
      (`/Game/Components/PowerComponent.StartComboAttack` (`self.PowerComponent`))
      (`self.PlayerAttackSound`))))

(event `Jump Attack`
  ;[1 1 1] Jump Attack
  (if (`self.CanAttack`)
    (`self.SetState` "NewEnumerator1")
    (`self.PlayJumpMontage`)
    (bind _asbp_player (cast `/Game/Player/BP_Player` (`self.GetOwner`)))
    (`Character.Jump` _asbp_player)
    (`self.PlayerSpecialAttackSound`)))

(event `SpinAttack`
  ;[1 1 1] Spin Attack
  (if (`self.CanAttack`)
    (`self.SetState` "NewEnumerator1")
    (`self.PlaySpinMontage`)
    (`self.PlayerSpecialAttackSound`)))

(event `PlayNextCombo`
  ;[1 1 1] Next Combo Attack
  (if (`self.ExistNextCombo`)
    (`self.PlayComboMontage`)
    (set `self.ExistNextCombo` false)
    (set `self.LastCombo` (== (- (`KismetArrayLibrary.Array_Length` (`self.ComboMontages`)) 1) (`self.ComboCount`)))
    (`self.PlayerAttackSound`)))

(fn `IsFalling`
  (returns (ReturnValue :type Boolean))
  (bind _asbp_player (cast `/Game/Player/BP_Player` (`self.GetOwner`)))
  (return (`NavMovementComponent.IsFalling` (`Character.CharacterMovement` _asbp_player))))

(fn `PlayComboMontage`
  (bind (_output_montage _output_playrate _output_startsectionname _output_canmove) (break `/Game/Struct/FComboMontage` (`|GetArrayItem` (`self.ComboMontages`) (`self.ComboCount`))))
  (bind _ascharacter (cast `Character` (`self.GetOwner`)))
  (`Character.PlayAnimMontage` _ascharacter _output_montage _output_playrate "None")
  (`self.SetCanMove` _output_canmove))

(fn `PlayerAttackSound`
  (`parent.PlayerAttackSound`)
  (if true
    (if (== (`self.SwordSoundIndex`) 0)
      (`GameplayStatics.PlaySound2D` "/Game/Sounds/MC_Link_Sword1_Cue.MC_Link_Sword1_Cue" 1.0 1.0 0.0 null null)
      (`/Engine/EditorBlueprintResources/StandardMacros.IncrementInt` (`self.SwordSoundIndex`))
      (elif (== (`self.SwordSoundIndex`) 1)
        (`GameplayStatics.PlaySound2D` "/Game/Sounds/MC_Link_Sword2_Cue.MC_Link_Sword2_Cue" 1.0 1.0 0.0 null null)
        (`/Engine/EditorBlueprintResources/StandardMacros.IncrementInt` (`self.SwordSoundIndex`))
        (elif (== (`self.SwordSoundIndex`) 2)
          (`GameplayStatics.PlaySound2D` "/Game/Sounds/MC_Link_Sword3_Cue.MC_Link_Sword3_Cue" 1.0 1.0 0.0 null null)
          (set `self.SwordSoundIndex` 0))))))

(fn `PlayerSpecialAttackSound`
  (`parent.PlayerSpecialAttackSound`)
  (if true
    (`GameplayStatics.PlaySound2D` "/Game/Sounds/MC_Link_Sword_Spin2_Cue.MC_Link_Sword_Spin2_Cue" 1.0 1.0 0.0 null null)))

(fn `PlayJumpMontage`
  (locals (Player :type "Character Object Reference"))
  (bind _ascharacter (cast `Character` (`self.GetOwner`)))
  (set `local.Player` _ascharacter)
  (`Pawn.AddMovementInput` (`local.Player`) (0.0 0.0 -1.0) 3000000.0 true)
  (`Character.PlayAnimMontage` (`local.Player`) "/Game/Character/Montages/SwordMontages/Falling_Attack_Montage.Falling_Attack_Montage" 1.0 "None")
  (`self.SetCanMove` false))

(fn `PlaySpinMontage`
  (bind _ascharacter (cast `Character` (`self.GetOwner`)))
  (`Character.PlayAnimMontage` _ascharacter "/Game/Character/Montages/SwordMontages/Standing_Melee_Attack_3_Montage.Standing_Melee_Attack_3_Montage" 1.0 "None")
  (`self.SetCanMove` false))

(fn `SendDamage`
  (params (OtherActor :type "Actor Object Reference"))
  (returns (Result :type Boolean))
  (locals (find :type Boolean))
  (for _array_element (`self.HittedCharacter`)
    (if (== _array_element (`local.OtherActor`))
      (set `local.find` true)
      (break)))
  (if (not (`local.find`))
    (bind _ascharacter (cast `Character` (`local.OtherActor`)))
    (`KismetArrayLibrary.Array_Add` (`self.HittedCharacter`) _ascharacter)
    (set `self.power` (`/Game/Components/PowerComponent.GetComboAttack` (`self.PowerComponent`) self (`self.ComboCount`)))
    (bind _result (`parent.SendDamage` (`local.OtherActor`)))
    (return _result)))

(fn `UserConstructionScript`
  (`parent.UserConstructionScript`))