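; Base weapon actor for characters, handling equipping, sheathing, damage and pickup into the player's WeaponInventory.
; State, combat style, movement lock and health changes are relayed to the owner through BP_IWeapon messages.
; Equipping and Sheathing play montages and switch rotation mode, Grab/UnGrab attach between hand and holster sockets, and Equipped/Sheathed restore state and movement.
; Attack, special attack and sound functions are empty stubs; SendDamage applies Power to other Characters.
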(event `Equipped`
  (`self.SetState` "NewEnumerator0")
  (`self.SetCanMove` true))

(event `Sheathed`
  (`self.SetState` "NewEnumerator0")
  (`self.SetCanMove` true)
  (`self.SetCombat` "NewEnumerator0"))

(event `Grab`
  (bind _ascharacter (cast `Character` (`self.GetOwner`)))
  (`self.K2_AttachToComponent` self (`Character.Mesh` _ascharacter) (`self.Socket`) "KeepRelative" "KeepRelative" "KeepRelative" true))

(event `UnGrab`
  (bind _ascharacter (cast `Character` (`self.GetOwner`)))
  (`self.K2_AttachToComponent` self (`Character.Mesh` _ascharacter) (`self.Holster`) "KeepRelative" "KeepRelative" "KeepRelative" true))

(event `/Game/BP_Interact.Interact`
  (bind _asbp_player (cast `/Game/Player/BP_Player` (`GameplayStatics.GetPlayerCharacter` 0)))
  (`/Game/Components/WeaponInventoryComponent.PickUp` (`/Game/Player/BP_Player.WeaponInventory` _asbp_player) (`self.WeaponData`))
  (`self.K2_DestroyActor`))

(event `On Selected`)

(event `Off Selected`)

(fn `Attack`)

(fn `CanAttack`
  (returns (Result :type Boolean))
  (return (and (`|EnumEquality` (`self.GetState`) "NewEnumerator0") (`|EnumEquality` (`self.GetCombat`) (`self.CombatStyle`)))))

(fn `DecreaseHealth`
  (params (Health :type "Float (double-precision)"))
  (returns (Result :type "Float (double-precision)"))
  (bind _returnvalue (`self.GetOwner`))
  (if (`KismetSystemLibrary.DoesImplementInterface` _returnvalue "/Game/BP_IWeapon.BP_IWeapon_C")
    (bind _result (message `/Game/BP_IWeapon.Weapon_DecreaseHealth` _returnvalue Health))
    (return _result)))

(fn `EndAttack`
  (`self.SetState` "NewEnumerator0"))

(fn `Equipping`
  (returns (ReturnValue :type "Float (double-precision)"))
  (`self.SetState` "NewEnumerator3")
  (`self.SetCanMove` false)
  (bind _ascharacter (cast `Character` (`self.GetOwner`)))
  (set `Pawn.bUseControllerRotationYaw` true _ascharacter)
  (set `CharacterMovementComponent.bOrientRotationToMovement` false (`Character.CharacterMovement` _ascharacter))
  (`self.SetCombat` (`self.CombatStyle`))
  (bind _returnvalue (`Character.PlayAnimMontage` _ascharacter (`self.DrawMontage`) 1.0 "None"))
  (return _returnvalue))

(fn `GetCanMove`
  (returns (CanMove :type Boolean))
  (bind _canmove (message `/Game/BP_IWeapon.GetWeapon_CanMove` (`self.GetOwner`)))
  (return _canmove))

(fn `GetCombat`
  (returns (Combat :type "/Game/Enums/ECombatStyle Enum"))
  (bind _returnvalue (`self.GetOwner`))
  (if (`KismetSystemLibrary.DoesImplementInterface` _returnvalue "/Game/BP_IWeapon.BP_IWeapon_C")
    (bind _combat (message `/Game/BP_IWeapon.GetWeapon_Combat` _returnvalue))
    (return _combat)))

(fn `GetState`
  (returns (state :type "/Game/Enums/EStateType Enum"))
  (bind _returnvalue (`self.GetOwner`))
  (if (`KismetSystemLibrary.DoesImplementInterface` _returnvalue "/Game/BP_IWeapon.BP_IWeapon_C")
    (bind _state (message `/Game/BP_IWeapon.GetWeapon_State` _returnvalue))
    (return _state)))

(fn `IncreaseHealth`
  (params (Health :type "Float (double-precision)"))
  (returns (Result :type "Float (double-precision)"))
  (bind _returnvalue (`self.GetOwner`))
  (if (`KismetSystemLibrary.DoesImplementInterface` _returnvalue "/Game/BP_IWeapon.BP_IWeapon_C")
    (bind _result (message `/Game/BP_IWeapon.Weapon_IncreaseHealth` _returnvalue Health))
    (return _result)))

(fn `PlayerAttackSound`
  (return))

(fn `PlayerSpecialAttackSound`
  (return))

(fn `SendDamage`
  (params (OtherActor :type "Actor Object Reference"))
  (returns (Result :type Boolean))
  (if (!= OtherActor (`self.GetOwner`))
    (bind _ascharacter (cast `Character` OtherActor)
      (:`then`
        (bind _returnvalue (`GameplayStatics.ApplyDamage` _ascharacter (`self.power`) (`self.GetInstigatorController` (`self.GetOwner`)) self))
        (`KismetSystemLibrary.PrintString` (`KismetStringLibrary.Conv_DoubleToString` _returnvalue))
        (return true))
      (:`CastFailed`
        (return false)))
    (else
      (return false))))

(fn `SetCanMove`
  (params (CanMove :type Boolean))
  (returns (Result :type Boolean))
  (bind _returnvalue (`self.GetOwner`))
  (if (`KismetSystemLibrary.DoesImplementInterface` _returnvalue "/Game/BP_IWeapon.BP_IWeapon_C")
    (bind _result (message `/Game/BP_IWeapon.SetWeapon_CanMove` _returnvalue CanMove))
    (return _result)))

(fn `SetCombat`
  (params (Combat :type "/Game/Enums/ECombatStyle Enum" :default "NewEnumerator0"))
  (returns (NewCombat :type "/Game/Enums/ECombatStyle Enum"))
  (bind _returnvalue (`self.GetOwner`))
  (if (`KismetSystemLibrary.DoesImplementInterface` _returnvalue "/Game/BP_IWeapon.BP_IWeapon_C")
    (bind _result (message `/Game/BP_IWeapon.SetWeapon_Combat` _returnvalue Combat))
    (return _result)))

(fn `SetState`
  (params (state :type "/Game/Enums/EStateType Enum" :default "NewEnumerator0"))
  (returns (Result :type "/Game/Enums/EStateType Enum"))
  (bind _result (message `/Game/BP_IWeapon.SetWeapon_State` (`self.GetOwner`) state))
  (return _result))

(fn `Sheathing`
  (returns (ReturnValue :type "Float (double-precision)"))
  (`self.SetState` "NewEnumerator2")
  (`self.SetCanMove` false)
  (bind _ascharacter (cast `Character` (`self.GetOwner`)))
  (set `Pawn.bUseControllerRotationYaw` false _ascharacter)
  (set `CharacterMovementComponent.bOrientRotationToMovement` true (`Character.CharacterMovement` _ascharacter))
  (bind _returnvalue (`Character.PlayAnimMontage` _ascharacter (`self.SheathMontage`) 1.0 "None"))
  (return _returnvalue))

(fn `Special Attack`)

(fn `UserConstructionScript`)