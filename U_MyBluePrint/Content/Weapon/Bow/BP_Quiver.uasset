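; BP_Quiver is a bow weapon quiver that displays nine arrows through an InstancedStaticMesh.
; On BeginPlay it gathers the Arrow1 to Arrow9 components and adds one mesh instance at each component's relative transform.
; The arrow components supply the layout for the instances, and the construction script is empty.
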(event `self.ReceiveBeginPlay`
  (bind _output_get (set `self.Arrows` (`|MakeArray` (`self.Arrow1`) (`self.Arrow2`) (`self.Arrow3`) (`self.Arrow4`) (`self.Arrow5`) (`self.Arrow6`) (`self.Arrow7`) (`self.Arrow8`) (`self.Arrow9`))))
  (for _array_element _output_get
    (`InstancedStaticMeshComponent.AddInstance` (`self.InstancedStaticMesh`) (`SceneComponent.GetRelativeTransform` _array_element))))

(fn `UserConstructionScript`)