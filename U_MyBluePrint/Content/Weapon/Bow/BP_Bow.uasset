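; Player bow weapon that handles aiming, firing arrows and equipping, with a quiver and hand arrow attached to character sockets.
; Attack or right-click zooms via spring arm and FOV timeline, while a Tick trace highlights the crosshair over damageable enemies.
; Release plays the bow montage; separate Shoot and EndShoot events fire and re-arm.
; Arrows launch from the bow socket toward a camera-trace target, so shots converge on screen center.
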(event `self.ReceiveTick`
  (params (DeltaSeconds :type "Float (single-precision)"))
  (bind _camera (`self.Get Camera`))
  (bind _returnvalue (`SceneComponent.K2_GetComponentLocation` _camera))
  (if (`self.IsAiming`)
    (bind (_outhit _returnvalue_2) (`KismetSystemLibrary.LineTraceSingleForObjects` :`Start` _returnvalue :`End` (+ _returnvalue (* (`SceneComponent.GetForwardVector` _camera) 3000.0)) :`ObjectTypes` (`|MakeArray` "ObjectTypeQuery3" :!type "EObjectTypeQuery Enum") :`TraceColor` (struct :`G` 1.0 :`A` 1.0) :`TraceHitColor` (struct :`R` 1.0 :`A` 1.0) :`DrawTime` 0.0))
    (if _returnvalue_2
      (bind _asbp_enemy (cast `/Game/Enemy/BP_Enemy` (`.HitActor` (`GameplayStatics.BreakHitResult` _outhit))))
      (if (`/Game/Enemy/BP_Enemy.CanDamaged` _asbp_enemy)
        (bind _asbp_player (cast `/Game/Player/BP_Player` (`self.GetOwner`)))
        (`/Game/Widgets/WB_CrossHair.On Focus` (`/Game/Player/BP_Player.CrossHair` _asbp_player)))
      (else
        (bind _asbp_player_2 (cast `/Game/Player/BP_Player` (`self.GetOwner`)))
        (`/Game/Widgets/WB_CrossHair.Off Focus` (`/Game/Player/BP_Player.CrossHair` _asbp_player_2))))))

(event `self.Attack`
  (if (`self.CanAttack`)
    (`self.Zoom In`)
    (`self.SetState` "NewEnumerator1")
    (`Widget.SetVisibility` (`self.Get CrossHair`) "Visible")
    (`self.SetActorHiddenInGame` (`self.HandArrow`) false)
    (set `self.IsPulled` true)))

(event `self.AttackRelease`
  (if (`self.ShootEnable`)
    (set `self.IsAiming` (`self.IsAiming`))
    (bind _ascharacter (cast `Character` (`self.GetOwner`)))
    (`Character.PlayAnimMontage` _ascharacter (`self.BowMontage`) 1.0 "None")
    (if (`self.IsAiming`)
      (set `self.IsPulled` false)
      (else
        (`self.Zoom Out`)
        (`self.SetState` "NewEnumerator0")
        (`Widget.SetVisibility` (`self.Get CrossHair`) "Hidden")
        (set `self.IsPulled` true)))))

(event `Shoot`
  (`|SpawnActorFromClass` (`self.Arrow`) (`KismetMathLibrary.MakeTransform` (`SceneComponent.GetSocketLocation` (`self.SkeletalMesh`) "Arrow_Socket") (`self.ShootTransform` (`SceneComponent.GetSocketLocation` (`self.SkeletalMesh`) "Arrow_Socket"))) "Undefined" "OverrideRootScale" self null)
  (set `self.ShootEnable` false)
  (`self.SetActorHiddenInGame` (`self.HandArrow`) true)
  (set `self.IsPulled` false))

(event `EndShoot`
  (set `self.ShootEnable` true)
  (`self.SetActorHiddenInGame` (`self.HandArrow`) false)
  (if (`self.IsAiming`)
    (set `self.IsPulled` true)
    (else
      (set `self.IsPulled` false))))

(event `self.Equipped`
  (bind _quiver (`self.Quiver`))
  (bind _handarrow (`self.HandArrow`))
  (`parent.Equipped`)
  (`|ExecutionSequence`
    (:`then_0`
      (`/Engine/EditorBlueprintResources/StandardMacros.IsValid` _quiver
        (:`Is Valid`
          (`self.SetActorHiddenInGame` _quiver false))
        (:`Is Not Valid`
          (`self.Make Quiver`))))
    (:`then_1`
      (`/Engine/EditorBlueprintResources/StandardMacros.IsValid` _handarrow
        (:`Is Valid`
          (`self.SetActorHiddenInGame` _handarrow false))
        (:`Is Not Valid`
          (`self.Make HandArrow`))))))

(event `self.Sheathed`
  (`parent.Sheathed`)
  (`self.SetActorHiddenInGame` (`self.Quiver`) true)
  (`self.SetActorHiddenInGame` (`self.HandArrow`) true))

(event `Zoom In`
  (bind _springarm (`self.Get SpringArm`))
  (set `self.IsAiming` true)
  (set `SpringArmComponent.TargetArmLength` 100.0 _springarm)
  (set `SpringArmComponent.SocketOffset` (0.0 30.0 0.0) _springarm)
  (`self.On Zoom In`))

(event `Zoom Out`
  (bind _springarm (`self.Get SpringArm`))
  (set `self.IsAiming` false)
  (set `SpringArmComponent.TargetArmLength` 300.0 _springarm)
  (set `SpringArmComponent.SocketOffset` (0.0 0.0 0.0) _springarm)
  (`self.On Zoom Out`))

(event `On Zoom In`
  (bind (_direction _zoom) (`Timeline|Zoom` :!label _label)
    (:`Update`
      (`CameraComponent.SetFieldOfView` (`self.Get Camera`) _zoom))))

(event `On Zoom Out`
  (goto _label :!via `Reverse`))

(event `self.RightClick`
  (`self.Zoom In`))

(event `self.RightClickRelease`
  (`self.Zoom Out`)
  (if (`|EnumEquality` (`self.GetState`) "NewEnumerator1")
    (`self.AttackRelease`)))

(fn `Get Camera`
  (returns (Camera :type "CameraComponent Object Reference"))
  (bind _asbp_player (cast `/Game/Player/BP_Player` (`self.GetOwner`)))
  (return (`/Game/Player/BP_Player.Camera` _asbp_player)))

(fn `Get CrossHair`
  (returns (CrossHair :type "/Game/Widgets/WB_CrossHair Object Reference"))
  (bind _asbp_player (cast `/Game/Player/BP_Player` (`self.GetOwner`)))
  (return (`/Game/Player/BP_Player.CrossHair` _asbp_player)))

(fn `Get SpringArm`
  (returns (SpringArm :type "SpringArmComponent Object Reference"))
  (bind _asbp_player (cast `/Game/Player/BP_Player` (`self.GetOwner`)))
  (return (`/Game/Player/BP_Player.SpringArm` _asbp_player)))

(fn `Make HandArrow`
  (bind _returnvalue (`|SpawnActorFromClass` (`self.Arrow`) (`KismetMathLibrary.MakeTransform` (0.0 0.0 0.0)) "Undefined" "OverrideRootScale" null null))
  (bind _output_get (set `self.HandArrow` _returnvalue))
  (`ActorComponent.SetActive` (`/Game/Weapon/Bow/BP_Arrow.ProjectileMovement` _output_get) false false)
  (`PrimitiveComponent.SetCollisionEnabled` (`/Game/Weapon/Bow/BP_Arrow.CollisionBox` _output_get) "NoCollision")
  (bind _ascharacter (cast `Character` (`self.GetOwner`)))
  (`self.K2_AttachToComponent` (`self.HandArrow`) (`Character.Mesh` _ascharacter) "Arrow_Socket" "KeepRelative" "KeepRelative" "KeepRelative" true))

(fn `Make Quiver`
  (bind _returnvalue (`|SpawnActorFromClass` "/Game/Weapon/Bow/BP_Quiver.BP_Quiver_C" (`KismetMathLibrary.MakeTransform` (0.0 0.0 0.0)) "Undefined" "OverrideRootScale" null null))
  (bind _output_get (set `self.Quiver` _returnvalue))
  (bind _ascharacter (cast `Character` (`self.GetOwner`)))
  (`self.K2_AttachToComponent` _output_get (`Character.Mesh` _ascharacter) "Quiver_Socket" "KeepRelative" "KeepRelative" "KeepRelative" true))

(fn `ShootTransform`
  (params (Location :type "Vector Structure"))
  (returns (ReturnValue :type "Rotator Structure"))
  (bind _asbp_player (cast `/Game/Player/BP_Player` (`self.GetOwner`)))
  (bind _camera (`/Game/Player/BP_Player.Camera` _asbp_player))
  (bind _returnvalue (`SceneComponent.K2_GetComponentLocation` _camera))
  (bind _returnvalue_2 (+ _returnvalue (* (`SceneComponent.GetForwardVector` _camera) 3000.0)))
  (bind (_outhit _returnvalue_3) (`KismetSystemLibrary.LineTraceSingle` :`Start` _returnvalue :`End` _returnvalue_2 :`TraceChannel` "TraceTypeQuery1" :`TraceColor` (struct :`G` 1.0 :`A` 1.0) :`TraceHitColor` (struct :`R` 1.0 :`A` 1.0)))
  (if _returnvalue_3
    (return (`KismetMathLibrary.FindLookAtRotation` (`local.Location`) (`.ImpactPoint` (`GameplayStatics.BreakHitResult` _outhit))))
    (else
      (return (`KismetMathLibrary.FindLookAtRotation` (`local.Location`) _returnvalue_2)))))

(fn `UserConstructionScript`
  (`parent.UserConstructionScript`))