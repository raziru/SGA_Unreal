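; BP_Arrow is the bow's arrow projectile, which damages actors it overlaps through its owning BP_Bow.
; Its BeginOverlap function ignores the bow's owner, gets single-attack power from PowerComponent, writes it to the bow and calls the bow's SendDamage.
; On successful damage it spawns the supplied explosion particle, offset from the hit actor and scaled to the arrow, then destroys itself.
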(fn `BeginOverlap`
  (params (`Other Actor` :type "Actor Object Reference") (Explosion :type "ParticleSystem Object Reference") (Location :type "Vector Structure") (Scale :type "Vector Structure") (Roatation :type "Rotator Structure"))
  (bind _asbp_bow (`self.GetOwnerToBow`))
  (if (!= `Other Actor` (`self.GetOwner` (`self.GetOwnerToBow`)))
    (bind _output_get (set `self.Power` (`/Game/Components/PowerComponent.GetSingleAttack` (`self.PowerComponent`) (`self.GetOwnerToBow`))))
    (set `/Game/Weapon/BP_Weapon.power` _output_get _asbp_bow)
    (bind _result (`/Game/Weapon/BP_Weapon.SendDamage` _asbp_bow (`local.Other Actor`)))
    (if _result
      (`GameplayStatics.SpawnEmitterAtLocation` (`local.Explosion`) (+ (`local.Location`) (`self.K2_GetActorLocation` (`local.Other Actor`))) (`local.Roatation`) (`self.GetActorScale3D`))
      (`self.K2_DestroyActor`))))

(fn `GetOwnerToArrow`)

(fn `GetOwnerToBow`
  (returns (`AsBP Bow` :type "/Game/Weapon/Bow/BP_Bow Object Reference"))
  (bind _asbp_bow (cast `/Game/Weapon/Bow/BP_Bow` (`self.GetOwner`)))
  (return _asbp_bow))

(fn `UserConstructionScript`)