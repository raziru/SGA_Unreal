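; BP_Item_Lantern is a lantern item that toggles a SpotLight component on top of its parent item behavior.
; The light starts hidden at BeginPlay, turns on with Equip or Use, and turns off with EndUse.
; UnEquip, selection events and construction only call the parent, so unequipping does not itself hide the light.
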(event `self.ReceiveBeginPlay`
  (`SceneComponent.SetVisibility` (`self.SpotLight`) false false))

(event `self.Use`
  (`parent.Use`)
  (`SceneComponent.SetVisibility` (`self.SpotLight`) true false))

(event `self.EndUse`
  (`parent.EndUse`)
  (`SceneComponent.SetVisibility` (`self.SpotLight`) false false))

(event `self.Off Selected`
  (`parent.Off Selected`))

(event `self.On Selected`
  (`parent.On Selected`))

(fn `Equip`
  (`parent.Equip`)
  (`SceneComponent.SetVisibility` (`self.SpotLight`) true false))

(fn `UnEquip`
  (`parent.UnEquip`))

(fn `UserConstructionScript`
  (`parent.UserConstructionScript`))