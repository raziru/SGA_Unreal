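; BP_Item is a base item actor that the player can pick up, equip, holster and use.
; Interact passes ItemData to the player's ItemInventory, then destroys the actor.
; Equip and UnEquip print the item's name and attach to the owning player's mesh at the Socket or Holster socket.
; Use and EndUse toggle IsUsed, while selection, effect, type and equip-end hooks are empty stubs.
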(event `On Selected`)

(event `Off Selected`)

(event `/Game/BP_Interact.Interact`
  (bind _asbp_player (cast `/Game/Player/BP_Player` (`GameplayStatics.GetPlayerCharacter` 0)))
  (`/Game/Components/InventoryComponent.PickUp` (`/Game/Player/BP_Player.ItemInventory` _asbp_player) (`self.ItemData`))
  (`self.K2_DestroyActor`))

(fn `EndEffect`)

(fn `EndEquip`)

(fn `EndUnEquip`)

(fn `EndUse`
  (set `self.isUsed` false))

(fn `Equip`
  (`KismetSystemLibrary.PrintString` (`KismetSystemLibrary.GetDisplayName` self))
  (`self.K2_AttachToComponent` self (`Character.Mesh` (`self.GetOwnerToPlayer`)) (`self.Socket`) "KeepRelative" "KeepRelative" "KeepRelative" true))

(fn `GetEffect`)

(fn `GetOwnerToPlayer`
  (returns (`AsBP Player` :type "/Game/Player/BP_Player Object Reference"))
  (bind _asbp_player (cast `/Game/Player/BP_Player` (`self.GetOwner`)))
  (return _asbp_player))

(fn `GetType`)

(fn `SetEffect`)

(fn `UnEquip`
  (`KismetSystemLibrary.PrintString` (`KismetSystemLibrary.GetDisplayName` self))
  (`self.K2_AttachToComponent` self (`Character.Mesh` (`self.GetOwnerToPlayer`)) (`self.Holster`) "KeepRelative" "KeepRelative" "KeepRelative" true))

(fn `Use`
  (set `self.isUsed` true))

(fn `UserConstructionScript`)