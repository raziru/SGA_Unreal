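; BP_TreasureChest_A is an interactable treasure chest that gives the player a lantern and a shield.
; On BeginPlay, StoreItem fills ItemList with one copy each of the lantern and shield data from ChestComponent.
; On Interact, it casts player character 0 to BP_Player and passes every entry to its ItemInventory's PickUp.
; The list is not cleared afterwards, and no opened state is tracked.
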(event `self.ReceiveBeginPlay`
  (`|ExecutionSequence`
    (:`then_0`
      (`self.StoreItem` (`/Game/Components/ChestComponent.LanternData` (`self.ChestComponent`)) 1))
    (:`then_1`
      (`self.StoreItem` (`/Game/Components/ChestComponent.ShieldData` (`self.ChestComponent`)) 1))))

(event `/Game/BP_Interact.Interact`
  (bind _asbp_player (cast `/Game/Player/BP_Player` (`GameplayStatics.GetPlayerCharacter` 0)))
  (for _array_element (`self.ItemList`)
    (`/Game/Components/InventoryComponent.PickUp` (`/Game/Player/BP_Player.ItemInventory` _asbp_player) _array_element)))

(fn `StoreItem`
  (params (ItemData :type "/Game/Struct/FItemData Structure") (Count :type Integer))
  (bind _result (`/Engine/EditorBlueprintResources/StandardMacros.DecrementInt` Count)
    (:`  `
      (for _ (range (+ _result 1))
        (`KismetArrayLibrary.Array_Add` (`self.ItemList`) ItemData)))))

(fn `UserConstructionScript`)