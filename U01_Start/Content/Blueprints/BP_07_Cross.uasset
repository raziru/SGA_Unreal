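; BP_07_Cross is a debug demo actor that visualizes the cross product between a Player and an Enemy actor.
; Each tick it draws arrows from the player for the direction to the enemy, the scaled forward vector, and their cross product.
; It also prints the player location, the cross vector and its dot with the player's up vector, a signed value indicating which side the enemy is on.
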(event `self.ReceiveTick`
  (params (DeltaSeconds :type "Float (single-precision)"))
  (bind _returnvalue (`self.GetPlayerLoaction`))
  (bind _returnvalue_2 (`self.GetPlayerLoaction`))
  (bind _returnvalue_3 (`self.GetPlayerLoaction`))
  (bind _returnvalue_4 (`KismetMathLibrary.Cross_VectorVector` (`self.GetPlayerForwardVector`) (`self.GetPlayerToEnemy`)))
  (`|ExecutionSequence`
    (:`then_0`
      (`KismetSystemLibrary.DrawDebugArrow` _returnvalue (+ _returnvalue (`self.GetPlayerToEnemy`)) 50.0 (struct :`R` 1.0 :`A` 1.0) 0.0 10.0))
    (:`then_1`
      (`KismetSystemLibrary.DrawDebugArrow` _returnvalue_3 (+ _returnvalue_3 (* (`self.GetPlayerForwardVector`) 300.0)) 50.0 (struct :`G` 1.0 :`B` 0.046318 :`A` 1.0) 0.0 10.0))
    (:`then_2`
      (`KismetSystemLibrary.DrawDebugArrow` _returnvalue_2 (+ _returnvalue_2 (`KismetMathLibrary.Cross_VectorVector` (`self.GetPlayerForwardVector`) (`self.GetPlayerToEnemy`))) 50.0 (struct :`R` 0.030084 :`B` 1.0 :`A` 1.0) 0.0 10.0))
    (:`then_3`
      (`KismetSystemLibrary.PrintString` (`KismetStringLibrary.Concat_StrStr` (`KismetStringLibrary.Conv_VectorToString` (`self.GetPlayerLoaction`)) "/" (`KismetStringLibrary.Conv_VectorToString` _returnvalue_4) "/" (`KismetStringLibrary.Conv_DoubleToString` (`KismetMathLibrary.Dot_VectorVector` (`self.GetPlayerUpVector`) _returnvalue_4)))))))

(fn `GetEnemyLocation`
  (returns (ReturnValue :type "Vector Structure"))
  (return (`self.K2_GetActorLocation` (`self.Enemy`))))

(fn `GetPlayerForwardVector`
  (returns (ReturnValue :type "Vector Structure"))
  (return (`self.GetActorForwardVector` (`self.Player`))))

(fn `GetPlayerLoaction`
  (returns (ReturnValue :type "Vector Structure"))
  (return (`self.K2_GetActorLocation` (`self.Player`))))

(fn `GetPlayerToEnemy`
  (returns (ReturnValue :type "Vector Structure"))
  (return (- (`self.K2_GetActorLocation` (`self.Enemy`)) (`self.K2_GetActorLocation` (`self.Player`)))))

(fn `GetPlayerUpVector`
  (returns (ReturnValue :type "Vector Structure"))
  (return (`self.GetActorUpVector` (`self.Player`))))

(fn `UserConstructionScript`)