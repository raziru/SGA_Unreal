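; Wizard warp skill that teleports the owning wizard to a cursor-targeted point on an actor named "Wall".
; Tick traces WorldStatic objects under the cursor and shows a targeting decal on walls while this skill is selected.
; Spell stores the hit location, moves the skill actor there, locks movement and plays the warp montage.
; EndSpell restores movement and relocates the wizard's owning actor to the stored location.
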(event `self.ReceiveTick`
  (params (DeltaSeconds :type "Float (single-precision)"))
  (bind _decal (`self.Decal`))
  (bind (_location _hitactor) (`self.GetCursorLocation`)
    (:`True`
      (if (== (`/Game/Weapons/Wizard/BP_Wizard.Skill` (`self.GetOwnerToWizard`)) self)
        (if (`KismetStringLibrary.EqualEqual_StrStr` (`KismetSystemLibrary.GetDisplayName` _hitactor) "Wall")
          (`SceneComponent.SetVisibility` _decal true false)
          (`SceneComponent.K2_SetWorldLocation` _decal _location false false)
          (else
            (`SceneComponent.SetVisibility` _decal false false :!label _label)))
        (else
          (goto _label))))
    (:`False`
      (goto _label))))

(event `self.Spell`
  (bind _wizard (`self.GetOwnerToWizard`))
  (bind (_location _hitactor) (`self.GetCursorLocation`)
    (:`True`
      (if (`KismetStringLibrary.EqualEqual_StrStr` (`KismetSystemLibrary.GetDisplayName` _hitactor) "Wall")
        (`self.K2_SetActorLocation` _location)
        (set `self.Location` _location)
        (`/Game/Weapons/BP_Weapon.SetCanMove` _wizard false) ; 타깃: 객체명->함수명과 같음
        (bind _ascharacter (cast `Character` (`self.GetOwner` _wizard)))
        (`Character.PlayAnimMontage` _ascharacter "/Game/Character/Montages/Wizard_Warp_Montage.Wizard_Warp_Montage" 1.0 "None")))
    (:`False`
      (`/Game/Weapons/BP_Weapon.SetCanMove` (`self.GetOwnerToWizard`) false)
      (`/Game/Weapons/BP_Weapon.SetState` (`self.GetOwnerToWizard`) "NewEnumerator0"))))

(event `self.EndSpell`
  (bind _wizard (`self.GetOwnerToWizard`))
  (`/Game/Weapons/BP_Weapon.SetCanMove` _wizard true)
  (`self.K2_SetActorLocation` (`self.GetOwner` _wizard) (`self.Location`) false false))

(fn `UserConstructionScript`
  (`parent.UserConstructionScript`))