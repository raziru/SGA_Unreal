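; Wizard weapon that casts spells through interchangeable skill actors.
; On BeginPlay it spawns Heal, Warp and Throw skills and attaches them to the owning Character's mesh, Heal and Throw at the hand socket.
; ChangeSkill swaps the active Skill, which receives focus changes on weapon selection and swap.
; Attack plays the throw montage and calls the active skill's Spell, while EndAttack runs the parent logic and ends the spell.
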(event `self.OnSelected`
  (`/Engine/EditorBlueprintResources/StandardMacros.IsValid` (`self.Skill`)
    (:`Is Valid`
      (`/Game/Weapons/Wizard/BP_WizardSkill.OnFocus` (`self.Skill`)))))

(event `self.OffSelected`
  (`/Engine/EditorBlueprintResources/StandardMacros.IsValid` (`self.Skill`)
    (:`Is Valid`
      (`/Game/Weapons/Wizard/BP_WizardSkill.OffFocus` (`self.Skill`)))))

(event `self.ReceiveBeginPlay`
  (set `self.CombatType` "NewEnumerator2")
  (`|ExecutionSequence`
    (:`then_0`
      (bind _returnvalue (`|SpawnActorFromClass` "/Game/Weapons/Wizard/BP_WizardSkill_Heal.BP_WizardSkill_Heal_C" (`KismetMathLibrary.MakeTransform` (0.0 0.0 0.0)) "Undefined" "OverrideRootScale" self null))
      (set `self.Heal` _returnvalue)
      (bind _ascharacter (cast `Character` (`self.GetOwner`)))
      (`self.K2_AttachToComponent` (`self.Heal`) (`Character.Mesh` _ascharacter) "Hand_FireBall" "KeepRelative" "KeepRelative" "KeepRelative" true))
    (:`then_1`
      (bind _returnvalue_2 (`|SpawnActorFromClass` "/Game/Weapons/Wizard/BP_WizardSkill_Warp.BP_WizardSkill_Warp_C" (`KismetMathLibrary.MakeTransform` (0.0 0.0 0.0)) "Undefined" "OverrideRootScale" self null))
      (set `self.Warp` _returnvalue_2)
      (bind _ascharacter_2 (cast `Character` (`self.GetOwner`)))
      (`self.K2_AttachToComponent` (`self.Warp`) (`Character.Mesh` _ascharacter_2) "None" "KeepRelative" "KeepRelative" "KeepRelative" true))
    (:`then_2`
      (bind _returnvalue_3 (`|SpawnActorFromClass` "/Game/Weapons/Wizard/BP_WizardSkill_Throw.BP_WizardSkill_Throw_C" (`KismetMathLibrary.MakeTransform` (0.0 0.0 0.0)) "Undefined" "OverrideRootScale" self null))
      (set `self.Throw` _returnvalue_3)
      (bind _ascharacter_3 (cast `Character` (`self.GetOwner`)))
      (`self.K2_AttachToComponent` (`self.Throw`) (`Character.Mesh` _ascharacter_3) "Hand_FireBall" "KeepRelative" "KeepRelative" "KeepRelative" true))))

(event `self.Attack`
  (if (and (`self.CanAttack`) (`KismetSystemLibrary.IsValid` (`self.Skill`)))
    (`self.SetState` "NewEnumerator4")
    (bind _ascharacter (cast `Character` (`self.GetOwner`)))
    (`Character.PlayAnimMontage` _ascharacter "/Game/Character/Montages/Wizard_Throw_Montage.Wizard_Throw_Montage" 1.0 "None")
    (`/Game/Weapons/Wizard/BP_WizardSkill.Spell` (`self.Skill`))))

(event `self.EndAttack`
  (`parent.EndAttack`)
  (`/Game/Weapons/Wizard/BP_WizardSkill.EndSpell` (`self.Skill`)))

(fn `ChangeSkill`
  (params (`new Skill` :type "/Game/Weapons/Wizard/BP_WizardSkill Object Reference"))
  (returns (Weapon :type "/Game/Weapons/BP_Weapon Object Reference"))
  (bind _new_skill (`local.new Skill`))
  (if (!= (`self.Skill`) `new Skill`)
    (`/Engine/EditorBlueprintResources/StandardMacros.IsValid` (`self.Skill`)
      (:`Is Valid`
        (`/Game/Weapons/Wizard/BP_WizardSkill.OffFocus` (`self.Skill`)))
      (:`Is Not Valid`
        _))
    (`/Engine/EditorBlueprintResources/StandardMacros.IsValid` _new_skill
      (:`Is Valid`
        (bind _output_get (set `self.Skill` _new_skill))
        (`/Game/Weapons/Wizard/BP_WizardSkill.OnFocus` _output_get))
      (:`Is Not Valid`
        (set `self.Skill` null)))))

(fn `UserConstructionScript`)